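; BP_Marble is a physics marble that a motion controller can pick up and drop, with a hover glow while not held.
; Each tick it plays impact sounds on sudden velocity changes, suppressed around grabs and throws, and starts rolling audio above a speed threshold.
; Inside gravity cubes, it disables gravity, raises damping and adds velocity along the closest cube's forward axis.
; A vector projection also pulls it toward that cube's center line, growing quadratically with distance.
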(event Custom|HandleHoverglow
  (params (Activate :type Boolean))
  ;[0 0 0] Handle Hoverglow.
  (if Activate
    (if (Variables|Default|GetIsGrabbed)
      (Rendering|Material|SetMaterial (Variables|Debug|GetStaticMeshComponent) 0 "/Game/GameElementBP/Material/M_Marble_Normal.M_Marble_Normal" :!label _label)
      (else
        (Rendering|Material|SetMaterial (Variables|Debug|GetStaticMeshComponent) 0 "/Game/GameElementBP/Material/M_Marble_Hover.M_Marble_Hover")))
    (else
      (goto _label))))

(event EventPickupFar
  (params (AttachTo :type Scene%20Component%20Object%20Reference))
  ;[0 0 0] Pickup marble
  (Physics|SetSimulatePhysics (Variables|Debug|GetStaticMeshComponent) false)
  (Transformation|AttachComponentToComponent (VehicleSound|GetRootComponent) AttachTo "None" "SnapToTarget" "KeepWorld" "KeepWorld" false)
  (Variables|Default|SetIsGrabbed true)
  (Variables|Default|SetWasPickedUp true))

(event EventPickup
  (params (AttachTo :type Scene%20Component%20Object%20Reference))
  ;[0 0 0] Pickup marble
  (Physics|SetSimulatePhysics (Variables|Debug|GetStaticMeshComponent) false)
  (Transformation|AttachComponentToComponent (VehicleSound|GetRootComponent) AttachTo "None" "KeepWorld" "KeepWorld" "KeepWorld" false)
  (Variables|Default|SetIsGrabbed true)
  (Variables|Default|SetWasPickedUp true))

(event EventDrop
  ;[0 0 0] Drop marble
  (Physics|SetSimulatePhysics (Variables|Debug|GetStaticMeshComponent) true)
  (Transformation|DetachFromActor "KeepWorld" "KeepWorld" "KeepWorld")
  (Variables|Default|SetIsGrabbed false))

(event EventTick
  (params (DeltaSeconds :type Float%20%28single-precision%29))
  (Utilities|FlowControl|Sequence
    (:then_0
      (CallFunction|HandleMarbleSound) ; Plays an impact and rolling sound.
    )
    (:then_1
      (CallFunction|HandleMarbleinGravityCube) ; Handles the forces of the gravity cubes that have an effect on the marble
    )))

(fn ConstructionScript)

(fn IsDeltaOverThreshold
  (params (Current :type Float%20%28single-precision%29) (Old :type Float%20%28single-precision%29))
  (Math|Float|CompareFloat (Math|Float|Absolute(Float) (- Current Old)) (Variables|Default|GetHitThreshold)
    (:>
      _)
    (:==
      _)
    (:<
      (return false)))
  (return true))

(fn IsDeltaOverThresholdVector
  (params (Current :type Vector) (Old :type Vector))
  (bind (_x _y _z) (Math|Vector|BreakVector Current))
  (bind (_x_2 _y_2 _z_2) (Math|Vector|BreakVector Old))
  (bind _isdifferenceoverthreshold (CallFunction|IsDeltaOverThreshold _x _x_2))
  (LocalVariables|Settemp (or _isdifferenceoverthreshold (LocalVariables|Gettemp)))
  (bind _isdifferenceoverthreshold_2 (CallFunction|IsDeltaOverThreshold _y _y_2))
  (LocalVariables|Settemp (or _isdifferenceoverthreshold_2 (LocalVariables|Gettemp)))
  (bind _isdifferenceoverthreshold_3 (CallFunction|IsDeltaOverThreshold _z _z_2))
  (bind _output_get (LocalVariables|Settemp (or _isdifferenceoverthreshold_3 (LocalVariables|Gettemp))))
  (return _output_get))

(fn IsWithinBounds
  (params (Actor :type Actor%20Object%20Reference) (Container :type Actor%20Object%20Reference))
  (return (Collision|IsOverlappingActor Actor Container :!class /Script/Engine.Actor)))

(fn CalcAccelarationtoBoxCenterLine
  (params (Box :type Actor%20Object%20Reference) (Marble :type Mesh%20Component%20Object%20Reference) (FocusingAccelerationAtBoxBorder :type Float%20%28single-precision%29))
  (bind _returnvalue (Transformation|GetActorRotation Box))
  (bind _returnvalue_2 (Math|Vector|GetForwardVector _returnvalue))
  (bind _returnvalue_3 (* _returnvalue_2 5.0))
  (LocalVariables|Set_marbleCenterLocation (Transformation|GetWorldLocation Marble))
  (LocalVariables|Set_boxCenterLocation (Transformation|GetActorLocation Box))
  ;[0 0 0] B  (VectorCenterLine -> the vector in the middle of the gravity cube in direction of the force)
  (LocalVariables|Set_startCenterLine (- (LocalVariables|Get_boxCenterLocation) _returnvalue_3))
  (LocalVariables|Set_vectorCenterLine (- (+ _returnvalue_3 (LocalVariables|Get_boxCenterLocation)) (- (LocalVariables|Get_boxCenterLocation) _returnvalue_3)))
  ;[0 0 0] A  (StartCenterLineToMarble)
  (LocalVariables|Set_startCenterLineToMarble (- (LocalVariables|Get_marbleCenterLocation) (LocalVariables|Get_startCenterLine)))
  ;[0 0 0] Projection of A on B
  (LocalVariables|Set_marbleProjectedOnCenterLine (+ (LocalVariables|Get_startCenterLine) (* (LocalVariables|Get_vectorCenterLine) (/ (Math|Vector|DotProduct (LocalVariables|Get_startCenterLineToMarble) (LocalVariables|Get_vectorCenterLine)) (Math|Float|Square (Math|Vector|VectorLength (LocalVariables|Get_vectorCenterLine)))))))
  (return (CallFunction|CalcFocusingAccelaration (- (LocalVariables|Get_marbleProjectedOnCenterLine) (LocalVariables|Get_marbleCenterLocation)) FocusingAccelerationAtBoxBorder)))

(fn CalcFocusingAccelaration
  (params (MarbleToCenterLine :type Vector) (FocusingAccelerationAtBoxBorder :type Float%20%28single-precision%29))
  (bind _returnvalue (Math|Vector|VectorLength MarbleToCenterLine))
  (return (* (* (/ MarbleToCenterLine _returnvalue) (Math|Float|Power _returnvalue 2.0)) (/ FocusingAccelerationAtBoxBorder (Math|Float|Power (LocalVariables|Get_halfBoxWidth) 2.0)))))

(fn GetClosestGravityCube
  (for _array_element (Collision|GetOverlappingActors (Variables|Debug|GetStaticMeshComponent) "/Game/GameElementBP/Cubes/NormalCube/BP_GridNormalCubeComplex.BP_GridNormalCubeComplex_C" :!class /Script/Engine.PrimitiveComponent)
    (bind _asbp_grid_normal_cube_complex (Utilities|Casting|CastToBP_GridNormalCubeComplex _array_element))
    (if (< (Math|Vector|VectorLength (- (Transformation|GetActorLocation self) (Transformation|GetActorLocation _asbp_grid_normal_cube_complex))) (LocalVariables|Get_ClosestGravityCubeDistance))
      (LocalVariables|Set_ClosestGravityCubeDistance (Math|Vector|VectorLength (- (Transformation|GetActorLocation self) (Transformation|GetActorLocation _asbp_grid_normal_cube_complex))))
      (LocalVariables|Set_ClosestGravityCube _asbp_grid_normal_cube_complex)))
  (return (LocalVariables|Get_ClosestGravityCube)))

(fn HandleMarbleSound
  (bind _returnvalue (Physics|GetPhysicsLinearVelocity (Variables|Debug|GetStaticMeshComponent) "None"))
  (LocalVariables|SetCurrVelocity _returnvalue)
  (Utilities|FlowControl|Sequence
    (:then_0
      (CallFunction|HandleImpactSound (LocalVariables|GetCurrVelocity)))
    (:then_1
      (CallFunction|HandleRollingSound (LocalVariables|GetCurrVelocity)))
    (:then_2
      (CallFunction|ResetWasPickedUp))))

(fn HandleMarbleinGravityCube
  (bind _closestgravitycube (CallFunction|GetClosestGravityCube))
  (if (Utilities|IsValid _closestgravitycube)
    (Variables|Default|SetGravityCube _closestgravitycube)
    (Physics|SetEnableGravity (Variables|Debug|GetStaticMeshComponent) false)
    ;[0 0 0] Force in direction of gravity box direction
    (Physics|SetPhysicsLinearVelocity (Variables|Debug|GetStaticMeshComponent) (* (Math|Vector|GetForwardVector (Transformation|GetActorRotation (Variables|Default|GetGravityCube))) (Variables|Default|GetDirectionalAcceleration)) true "None")
    ;[0 0 0] Force in direction of the center of the gravity box
    (Physics|SetPhysicsLinearVelocity (Variables|Debug|GetStaticMeshComponent) (CallFunction|CalcAccelarationtoBoxCenterLine (Variables|Default|GetGravityCube) (Variables|Debug|GetStaticMeshComponent) 5.0) true "None")
    (Class|PrimitiveComponent|SetLinearDamping (Variables|Debug|GetStaticMeshComponent self) 6.0)
    (else
      ;[0 0 0] Resets the gravity of the marble
      (Physics|SetEnableGravity (Variables|Debug|GetStaticMeshComponent) true)
      (Variables|Default|SetGravityCube 0)
      (Class|PrimitiveComponent|SetLinearDamping (Variables|Debug|GetStaticMeshComponent self) 0.01))))

(fn ResetWasPickedUp
  ;[0 0 0] Reset WasPickedUp variable after one tick.
  (if (and (Math|Boolean|Equal(Boolean) (Variables|Default|GetIsGrabbed) false) (Math|Boolean|Equal(Boolean) (Variables|Default|GetWasPickedUp) true))
    (Variables|Default|SetWasPickedUp false)))

(fn HandleRollingSound
  (params (CurrVelocity :type Vector))
  ;[0 0 0] Rolling
  (Audio|Components|Audio|SetVolumeMultiplier (Variables|Default|GetMarbleRollingQuiet) (* 2 (Variables|Default|GetRollingSoundDampening)) :!class /Script/Engine.AudioComponent)
  (if (Variables|Default|GetIsGrabbed)
    (Audio|Components|Audio|Stop (Variables|Default|GetMarbleRollingQuiet) :!label _label)
    (else
      (Variables|Default|GetGravityCube
        (:then
          (goto _label))
        (:else
          (if (> (Math|Vector|VectorLengthXY CurrVelocity) (Variables|Default|GetRollingSoundVelocityThreshold))
            (if (not (Audio|Components|Audio|IsPlaying (Variables|Default|GetMarbleRollingQuiet)))
              (Audio|Components|Audio|Play (Variables|Default|GetMarbleRollingQuiet) 0.0))))))))

(fn HandleImpactSound
  (params (CurrVelocity :type Vector))
  ;[0 0 0] Impact
  (bind _isoverthreshold (CallFunction|IsDeltaOverThresholdVector CurrVelocity (LocalVariables|GetOldVelocity))) ; Checks, if there was a rapid velocity change.
  (LocalVariables|SetOldVelocity CurrVelocity)
  (if _isoverthreshold
    ;;[0 0 0] Currently not in hand and neither one tick before (throwing) to avoid impact sound on throw.
    (if (and (not (Variables|Default|GetWasPickedUp)) (not (Variables|Default|GetIsGrabbed)))
      (Audio|Components|Audio|SetVolumeMultiplier (Variables|Default|GetImpactOnTile) (/ (Math|Vector|VectorLength (LocalVariables|GetOldVelocity)) 4e+01) :!class /Script/Engine.AudioComponent)
      (Audio|Components|Audio|Play (Variables|Default|GetImpactOnTile) 0.0))))