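; BP_GridEndCubeComplex is a grabbable cube that replaces itself with a simpler BP_GridEndCube when picked up.
; On Pickup it spawns that cube at its own transform and records it as the motion controller's AttachedActor.
; It then disables the new cube's physics and constraint mode, attaches its mesh to the hand component, enables tick, flags it as grabbed, and destroys itself.
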(event EventPickup
  (params (AttachTo :type Scene%20Component%20Object%20Reference))
  (Variables|Default|SetPosition (Transformation|GetActorLocation))
  (Variables|Default|SetRotation (Transformation|GetActorRotation))
  (bind _returnvalue (Game|SpawnActorfromClass "/Game/GameElementBP/Cubes/EndCube/BP_GridEndCube.BP_GridEndCube_C" (Math|Transform|MakeTransform (Variables|Default|GetPosition) (Variables|Default|GetRotation)) "Undefined" 0 0))
  (bind _asbp_motion_controller (Utilities|Casting|CastToBP_MotionController (Components|GetOwner AttachTo)))
  (Variables|/Game/VirtualRealityBP/Blueprints/BP_MotionController.BP_MotionController_C|SetAttachedActor _asbp_motion_controller _returnvalue)
  (Physics|SetSimulatePhysics (Variables|/Script/Engine.StaticMeshActor|GetStaticMeshComponent _returnvalue) false)
  (Transformation|AttachComponentToComponent (Variables|/Script/Engine.StaticMeshActor|GetStaticMeshComponent _returnvalue) AttachTo "None" "KeepWorld" "KeepWorld" "KeepWorld" false)
  (Class|PrimitiveComponent|SetConstraintMode (Variables|/Script/Engine.StaticMeshActor|GetStaticMeshComponent _returnvalue) "None")
  (Actor|Tick|SetActorTickEnabled _returnvalue true)
  (Variables|/Game/GameElementBP/BP_GridCube.BP_GridCube_C|SetIsGrabbed _returnvalue true)
  (Actor|DestroyActor))

(fn ConstructionScript
  (|CallParentFunction))