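; BP_GridGravityCubeComplex is the complex form of the gravity grid cube, which can be grabbed with a motion controller.
; Pickup and PickupFar spawn a simple BP_GridGravityCube at its transform for that controller, keeping world position or snapping to it respectively.
; Tick is empty.
; An unconnected leftover would add distance-squared velocity to overlapping grid cubes, directed away from this cube, with debug arrows.
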(event EventTick
  (params (DeltaSeconds :type Float%20%28single-precision%29))
  ;[0 0 0] TODO: Den anderen Cubes hinzufügen ????
)

(event EventPickupFar
  (params (AttachTo :type Scene%20Component%20Object%20Reference))
  (CallFunction|SpawnSimpleVersion "SnapToTarget" (Transformation|GetActorLocation) (Transformation|GetActorRotation) AttachTo "/Game/GameElementBP/Cubes/GravityCube/BP_GridGravityCube.BP_GridGravityCube_C"))

(event EventPickup
  (params (AttachTo :type Scene%20Component%20Object%20Reference))
  (CallFunction|SpawnSimpleVersion "KeepWorld" (Transformation|GetActorLocation) (Transformation|GetActorRotation) AttachTo "/Game/GameElementBP/Cubes/GravityCube/BP_GridGravityCube.BP_GridGravityCube_C"))

(fn ConstructionScript
  (|CallParentFunction))