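; Grabbable cube that animates into the motion controller on pickup, snaps beside other pickup cubes and plays velocity-scaled impact sounds.
; While held, Tick line-traces to find the nearest cube within two widths and shows a ghost at the hit face, rotated in 90-degree steps.
; Drop applies that snap, then overwrites rotation with a hard-coded debug value.
; Tick re-applies the stored pre-override transform every frame to hold snapped cubes.
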(event EventTick
  (params (DeltaSeconds :type Float%20%28single-precision%29))
  (if (Variables|Default|GetIsSnapped)
    ;[1 1 1] Resets the snapped transform every frame (if snapped).
    (Transformation|SetActorTransform (Variables|Default|GetSnappedLocation))
    (Physics|SetPhysicsLinearVelocity (Variables|Debug|GetStaticMeshComponent) "0, 0, 0" false "None")
    (elif (Variables|Default|GetIsPickedUp)
      (bind (_closestobject _closesthitlocation) (CallFunction|FindClosestPickupCube))
      (if (!= _closestobject 0)
        (bind (_xoffset _yoffset _zoffset) (CallFunction|SetOffsetOfCollisionSide _closesthitlocation _closestobject))
        (if (Variables|Default|GetIsGhostSpawned)
          (Transformation|SetActorTransform (Variables|Default|GetSpawnedGhost) (Transformation|GetActorTransform _closestobject))
          (else
            (bind _returnvalue (Game|SpawnActorfromClass "/Game/GameElementBP/BP_CurveCubeGhost.BP_CurveCubeGhost_C" (Transformation|GetActorTransform _closestobject) "Undefined" 0 0)) ; TODO: Spawn Transform anpassen
            (Variables|Default|SetSpawnedGhost _returnvalue)
            (Variables|Default|SetIsGhostSpawned true)))
        (Transformation|AddActorLocalOffset (Variables|Default|GetSpawnedGhost) (Math|Vector|MakeVector _xoffset _yoffset _zoffset) false false)
        (bind (_xrotation _yrotation _zrotation) (CallFunction|CalculateRotationOfSnappingObject3 _closestobject))
        (Transformation|SetActorRotation (Variables|Default|GetSpawnedGhost) (Math|Rotator|MakeRotator _xrotation _yrotation _zrotation))
        (else
          ;[1 1 1] Destroys the Ghost Actor, when distance is too big again.
          (if (Variables|Default|GetIsGhostSpawned)
            (Actor|DestroyActor (Variables|Default|GetSpawnedGhost))
            (Variables|Default|SetIsGhostSpawned false)))))))

(event EventPickup
  (params (AttachTo :type Scene%20Component%20Object%20Reference))
  (bind _returnvalue (Transformation|GetWorldTransform AttachTo))
  ;[1 1 1] Grab animation, buggy when player interacts with it during animation
  (Components|MoveComponentTo (Variables|Debug|GetStaticMeshComponent) (.location _returnvalue) (.rotation _returnvalue) false false (Variables|Default|GetGrabAnimationTime) false)
  (Physics|SetSimulatePhysics (Variables|Debug|GetStaticMeshComponent) false)
  (Transformation|AttachComponentToComponent (VehicleSound|GetRootComponent) AttachTo "None" "SnapToTarget" "SnapToTarget" "KeepWorld" false)
  (Variables|Default|SetIsPickedUp true)
  (Variables|Default|SetIsSnapped false)
  (Rendering|SetVisibility (Variables|Default|GetHoverGlow) false false))

(event Collision|EventHit
  (params (MyComp :type Primitive%20Component%20Object%20Reference) (Other :type Actor%20Object%20Reference) (OtherComp :type Primitive%20Component%20Object%20Reference) (bSelfMoved :type Boolean) (HitLocation :type Vector :default "0, 0, 0") (HitNormal :type Vector :default "0, 0, 0") (NormalImpulse :type Vector :default "0, 0, 0") (Hit :type Hit%20Result%20Structure%20%28by%20ref%29))
  (bind _returnvalue (Transformation|GetVelocity))
  (bind _returnvalue_2 (Math|Vector|VectorLength _returnvalue))
  (bind _returnvalue_3 (/ _returnvalue_2 6e+01))
  (bind _returnvalue_4 (Math|Float|Clamp(Float) _returnvalue_3 0.0 1.4))
  ;[1 1 1] Sound bei Kollision
  (Math|Float|CompareFloat (Math|Vector|VectorLength HitLocation) 1e+03
    (:>
      _)
    (:==
      _)
    (:<
      ;[1 1 1] Light Impact
      (Utilities|FlowControl|DoOnce false :!label _label
        (:Completed
          (Audio|PlaySoundatLocation "/Game/Audio/A_wood-hit-on-hard-floor-short_Cue.A_wood-hit-on-hard-floor-short_Cue" HitLocation "0, 0, 0" _returnvalue_4 1.0 0.0 0 0 0)
          (Utilities|FlowControl|Delay 0.190113)
          (goto _label Reset)))))
  ;[1 1 1] Heavy Impact
  (Utilities|FlowControl|DoOnce false :!label _label_2
    (:Completed
      (Audio|PlaySoundatLocation "/Game/Audio/A_wood-hit-on-hard-floor-short_Cue.A_wood-hit-on-hard-floor-short_Cue" HitLocation "0, 0, 0" _returnvalue_4 1.0 0.0 0 0 0)
      (Utilities|FlowControl|Delay 0.190113)
      (goto _label_2 Reset))))

(event EventDrop
  (if (Variables|Default|GetIsGhostSpawned)
    (Actor|DestroyActor (Variables|Default|GetSpawnedGhost))
    (Variables|Default|SetIsGhostSpawned false))
  (Physics|SetSimulatePhysics (Variables|Debug|GetStaticMeshComponent) true)
  (Transformation|DetachFromActor "KeepWorld" "KeepWorld" "KeepWorld")
  (Variables|Default|SetIsPickedUp false)
  (bind (_closestobject _closesthitlocation) (CallFunction|FindClosestPickupCube))
  (if (!= _closestobject 0)
    (Variables|Default|SetIsSnapped true)
    (bind (_xoffset _yoffset _zoffset) (CallFunction|SetOffsetOfCollisionSide _closesthitlocation _closestobject))
    (bind (_xrotation _yrotation _zrotation) (CallFunction|CalculateRotationOfSnappingObject3 _closestobject))
    (Transformation|SetActorTransform (Transformation|GetActorTransform _closestobject))
    (Transformation|AddActorLocalOffset (Math|Vector|MakeVector _xoffset _yoffset _zoffset) false false)
    (Transformation|SetActorRotation (Math|Rotator|MakeRotator _xrotation _yrotation _zrotation))
    (Variables|Default|SetSnappedLocation (Transformation|GetActorTransform))
    (Physics|SetPhysicsLinearVelocity (Variables|Debug|GetStaticMeshComponent) "0, 0, 0" false "None")
    (Audio|PlaySoundatLocation "/Game/Audio/A_BuildBlock_Cue.A_BuildBlock_Cue" (Transformation|GetActorLocation) "0, 0, 0" 1.0 1.0 0.0 0 0 0)
    (Development|PrintString (Utilities|String|ToString(Rotator) (Transformation|GetActorRotation)) true true "(R=1.000000,G=0.000000,B=0.120205,A=1.000000)" 2e+01)
    (Transformation|SetActorRotation "360.000000,181.000000,270.000000")
    (Development|PrintString (Utilities|String|ToString(Rotator) (Transformation|GetActorRotation)) true true "(R=0.000000,G=0.660000,B=1.000000,A=1.000000)" 2e+01)))

(fn ConstructionScript)

(fn GetCubeWidth
  (return (* (* (.x (Transformation|GetActorScale3D)) (.x (.Max (Components|StaticMesh|GetLocalBounds (Variables|Debug|GetStaticMeshComponent))))) 2.0)))

(fn SetOffsetOfCollisionSide
  (params (HitLocation :type Vector) (ClosestObject :type Actor%20Object%20Reference))
  (bind _returnvalue (Transformation|GetActorTransform ClosestObject))
  (bind _returnvalue_2 (Math|Transform|InverseTransformLocation _returnvalue HitLocation))
  (bind _returnvalue_3 (Math|Float|Absolute(Float) (.x _returnvalue_2)))
  (bind _returnvalue_4 (Math|Float|Absolute(Float) (.y _returnvalue_2)))
  (bind _returnvalue_5 (Math|Float|Absolute(Float) (.z _returnvalue_2)))
  (bind (_xoffset _yoffset _zoffset) (CallFunction|CalculateOffsetsfromHitSide (.x _returnvalue_2) (.y _returnvalue_2) (.z _returnvalue_2)))
  ;[1 1 1] Calculates the hit side (line trace from Self to Closest Object) and only sets the Offset of the hit side.
  (Math|Float|CompareFloat _returnvalue_3 _returnvalue_4
    (:>
      (Math|Float|CompareFloat _returnvalue_3 _returnvalue_5 :!label _label
        (:>
          (bind _output_get (LocalVariables|Set_XOffset _xoffset :!label _label_2)))
        (:==
          (goto _label_2))
        (:<
          (bind _output_get_2 (LocalVariables|Set_ZOffset _zoffset :!label _label_3)))))
    (:==
      (goto _label))
    (:<
      (Math|Float|CompareFloat _returnvalue_4 _returnvalue_5
        (:>
          (bind _output_get_3 (LocalVariables|Set_YOffset _yoffset)))
        (:==
          (goto _label_3))
        (:<
          (goto _label_3)))))
  (return _output_get _output_get_3 _output_get_2))

(fn CalculateOffsetsfromHitSide
  (params (LocalHitX :type Float%20%28single-precision%29) (LocalHitY :type Float%20%28single-precision%29) (LocalHitZ :type Float%20%28single-precision%29))
  ;[1 1 1] Calculates the offset for all three dimensions.
  (bind _returnvalue (CallFunction|GetCubeWidth))
  (return (* (Math|Float|Sign(Float) LocalHitX) _returnvalue) (* (Math|Float|Sign(Float) LocalHitY) _returnvalue) (* (Math|Float|Sign(Float) LocalHitZ) _returnvalue)))

(fn FindClosestPickupCube
  (LocalVariables|Set_ShortestDistance 999999995904.0)
  (bind _outactors (Actor|GetAllActorswithInterface "/Game/VirtualRealityBP/Blueprints/PickupActorInterface.PickupActorInterface_C"))
  (for _array_element _outactors
    (bind _outhit (Collision|LineTraceForObjects (Transformation|GetActorLocation self) (Transformation|GetActorLocation _array_element) (Utilities|Array|MakeArray "ObjectTypeQuery4") false 0 "None"))
    (if (.bBlockingHit (Collision|BreakHitResult _outhit))
      (if (.bSuccess (Utilities|Casting|CastToBP_PickupCube (.HitActor (Collision|BreakHitResult _outhit))))
        ;[1 1 1] Berechnet die Länge von aktuellem Standpunkt zum Hitpunkt
        (bind _output_get (LocalVariables|Set_HitLocation (.Location (Collision|BreakHitResult _outhit))))
        (LocalVariables|Set_CurrDistance (Math|Vector|VectorLength (- _output_get (Transformation|GetActorLocation self))))
        ;[1 1 1] Wenn es der naheste Schnittpunkt ist dann wird das getroffene Objekt und die minimale Distanz gesetzt!
        (if (and (< (LocalVariables|Get_CurrDistance) (LocalVariables|Get_ShortestDistance)) (!= (LocalVariables|Get_CurrDistance) 0.0))
          (bind _returnvalue (CallFunction|GetCubeWidth))
          (if (< (LocalVariables|Get_CurrDistance) (* _returnvalue 2.0))
            (LocalVariables|Set_ClosestObject (.AsBP%20Pickup%20Cube (Utilities|Casting|CastToBP_PickupCube (.HitActor (Collision|BreakHitResult _outhit)))))
            (LocalVariables|Set_ShortestDistance (LocalVariables|Get_CurrDistance))
            (LocalVariables|Set_ClosestHitLocation (LocalVariables|Get_HitLocation)))))))
  (return (LocalVariables|Get_ClosestObject) (LocalVariables|Get_ClosestHitLocation)))

(fn CalculateRotationOfSnappingObject
  (params (ClosestObject :type Actor%20Object%20Reference))
  (bind _returnvalue (Transformation|GetActorRotation ClosestObject))
  (bind _returnvalue_2 (Transformation|GetActorRotation))
  (bind _rotationindegree (CallFunction|ConvertRotationtoRotationinDegree (Math|Float|Round (.roll _returnvalue))))
  (bind _rotationindegree_2 (CallFunction|ConvertRotationtoRotationinDegree (Math|Float|Round (.pitch _returnvalue))))
  (bind _rotationindegree_3 (CallFunction|ConvertRotationtoRotationinDegree (Math|Float|Round (.yaw _returnvalue))))
  (bind _rotationindegree_4 (CallFunction|ConvertRotationtoRotationinDegree (Math|Float|Round (.roll _returnvalue_2))))
  (bind _rotationindegree_5 (CallFunction|ConvertRotationtoRotationinDegree (Math|Float|Round (.pitch _returnvalue_2))))
  (bind _rotationindegree_6 (CallFunction|ConvertRotationtoRotationinDegree (Math|Float|Round (.yaw _returnvalue_2))))
  (LocalVariables|Set_Temp_X (/ _rotationindegree_4 90))
  (LocalVariables|Set_Temp_Y (/ _rotationindegree_5 90))
  (LocalVariables|Set_Temp_Z (/ _rotationindegree_6 90))
  (Math|Integer|CompareInt (Math|Integer|%(Integer) _rotationindegree_4 90) 45
    (:>
      (bind _output_get (LocalVariables|Set_MultiplyBy90Amount_X (+ (LocalVariables|Get_Temp_X) 1) :!label _label)))
    (:==
      (goto _label))
    (:<
      _))
  (Math|Integer|CompareInt (Math|Integer|%(Integer) _rotationindegree_5 90) 45
    (:>
      (bind _output_get_2 (LocalVariables|Set_MultiplyBy90Amount_Y (+ (LocalVariables|Get_Temp_Y) 1) :!label _label_2)))
    (:==
      (goto _label_2))
    (:<
      _))
  (Math|Integer|CompareInt (Math|Integer|%(Integer) _rotationindegree_6 90) 45
    (:>
      _)
    (:==
      _))
  (bind _output_get_3 (LocalVariables|Set_MultiplyBy90Amount_Z (+ (LocalVariables|Get_Temp_Z) 1)))
  (return (Math|Conversions|ToFloat(Integer) (+ (Math|Integer|%(Integer) _rotationindegree 90) (* _output_get 90))) (Math|Conversions|ToFloat(Integer) (+ (Math|Integer|%(Integer) _rotationindegree_2 90) (* _output_get_2 90))) (Math|Conversions|ToFloat(Integer) (+ (Math|Integer|%(Integer) _rotationindegree_3 90) (* _output_get_3 90)))))

(fn ConvertRotationtoRotationinDegree
  (params (Rotation :type Integer))
  (Math|Integer|CompareInt (Class|KismetMathLibrary|SignOfInteger Rotation)
    (:>
      (LocalVariables|SetReturnValue Rotation :!label _label))
    (:==
      (goto _label))
    (:<
      (LocalVariables|SetReturnValue (+ (- 180 (Math|Integer|Absolute(Integer) Rotation)) 180))))
  (return (LocalVariables|GetReturnValue)))

(fn CalculateRotationOfSnappingObject2
  (params (ClosestObject :type Actor%20Object%20Reference))
  (bind _returnvalue (Transformation|GetActorRotation))
  (bind _rotationindegree (CallFunction|ConvertRotationtoRotationinDegree (Math|Float|Round (.roll _returnvalue))))
  (bind _rotationindegree_2 (CallFunction|ConvertRotationtoRotationinDegree (Math|Float|Round (.pitch _returnvalue))))
  (bind _rotationindegree_3 (CallFunction|ConvertRotationtoRotationinDegree (Math|Float|Round (.yaw _returnvalue))))
  (LocalVariables|Set_Temp_X (/ _rotationindegree 90))
  (LocalVariables|Set_Temp_Y (/ _rotationindegree_2 90))
  (LocalVariables|Set_Temp_Z (/ _rotationindegree_3 90))
  (Math|Integer|CompareInt (Math|Integer|%(Integer) _rotationindegree 90) 45
    (:>
      (bind _output_get (LocalVariables|Set_MultiplyBy90Amount_X (+ (LocalVariables|Get_Temp_X) 1) :!label _label)))
    (:==
      (goto _label))
    (:<
      _))
  (Math|Integer|CompareInt (Math|Integer|%(Integer) _rotationindegree_2 90) 45
    (:>
      (bind _output_get_2 (LocalVariables|Set_MultiplyBy90Amount_Y (+ (LocalVariables|Get_Temp_Y) 1) :!label _label_2)))
    (:==
      (goto _label_2))
    (:<
      _))
  (Math|Integer|CompareInt (Math|Integer|%(Integer) _rotationindegree_3 90) 45
    (:>
      _)
    (:==
      _))
  (bind _output_get_3 (LocalVariables|Set_MultiplyBy90Amount_Z (+ (LocalVariables|Get_Temp_Z) 1)))
  (return (Math|Conversions|ToFloat(Integer) (* _output_get 90)) (Math|Conversions|ToFloat(Integer) (* _output_get_2 90)) (Math|Conversions|ToFloat(Integer) (* _output_get_3 90))))

(fn CalculateRotationOfSnappingObject3
  (params (ClosestObject :type Actor%20Object%20Reference))
  (bind _returnvalue (Transformation|GetActorRotation ClosestObject))
  (bind _returnvalue_2 (Transformation|GetActorRotation))
  (bind _rotationindegree (CallFunction|ConvertRotationtoRotationinDegree (Math|Float|Round (.roll _returnvalue))))
  (bind _rotationindegree_2 (CallFunction|ConvertRotationtoRotationinDegree (Math|Float|Round (.pitch _returnvalue))))
  (bind _rotationindegree_3 (CallFunction|ConvertRotationtoRotationinDegree (Math|Float|Round (.yaw _returnvalue))))
  (bind _rotationindegree_4 (CallFunction|ConvertRotationtoRotationinDegree (Math|Float|Round (.roll _returnvalue_2))))
  (bind _rotationindegree_5 (CallFunction|ConvertRotationtoRotationinDegree (Math|Float|Round (.pitch _returnvalue_2))))
  (bind _rotationindegree_6 (CallFunction|ConvertRotationtoRotationinDegree (Math|Float|Round (.yaw _returnvalue_2))))
  (Math|Integer|CompareInt (Class|KismetMathLibrary|SignOfInteger (- _rotationindegree_4 (Math|Integer|%(Integer) _rotationindegree 90)))
    (:>
      (Math|Integer|CompareInt (Math|Integer|%(Integer) (- _rotationindegree_4 (Math|Integer|%(Integer) _rotationindegree 90)) 90) 45 :!label _label
        (:>
          (LocalVariables|Set_90or0_X 90 :!label _label_2))
        (:==
          (goto _label_2))
        (:<
          (LocalVariables|Set_90or0_X 0))))
    (:==
      (goto _label))
    (:<
      (Math|Integer|CompareInt (Math|Integer|%(Integer) (- _rotationindegree_4 (Math|Integer|%(Integer) _rotationindegree 90)) 90) -45
        (:>
          (LocalVariables|Set_Negative90or0_X 0 :!label _label_3))
        (:==
          (goto _label_3))
        (:<
          (LocalVariables|Set_Negative90or0_X -90)))))
  (bind _output_get (LocalVariables|Set_Temp_X (+ (LocalVariables|Get_90or0_X) (LocalVariables|Get_Negative90or0_X))))
  (Math|Integer|CompareInt (Class|KismetMathLibrary|SignOfInteger (- _rotationindegree_5 (Math|Integer|%(Integer) _rotationindegree_2 90)))
    (:>
      (Math|Integer|CompareInt (Math|Integer|%(Integer) (- _rotationindegree_5 (Math|Integer|%(Integer) _rotationindegree_2 90)) 90) 45 :!label _label_4
        (:>
          (LocalVariables|Set_90or0_Y 90 :!label _label_5))
        (:==
          (goto _label_5))
        (:<
          (LocalVariables|Set_90or0_Y 0))))
    (:==
      (goto _label_4))
    (:<
      (Math|Integer|CompareInt (Math|Integer|%(Integer) (- _rotationindegree_5 (Math|Integer|%(Integer) _rotationindegree_2 90)) 90) -45
        (:>
          (LocalVariables|Set_Negative90or0_Y 0 :!label _label_6))
        (:==
          (goto _label_6))
        (:<
          (LocalVariables|Set_Negative90or0_Y -90)))))
  (bind _output_get_2 (LocalVariables|Set_Temp_Y (+ (LocalVariables|Get_90or0_Y) (LocalVariables|Get_Negative90or0_Y))))
  (Math|Integer|CompareInt (Class|KismetMathLibrary|SignOfInteger (- _rotationindegree_6 (Math|Integer|%(Integer) _rotationindegree_3 90)))
    (:>
      (Math|Integer|CompareInt (Math|Integer|%(Integer) (- _rotationindegree_6 (Math|Integer|%(Integer) _rotationindegree_3 90)) 90) 45 :!label _label_7
        (:>
          (LocalVariables|Set_90or0_Z 90 :!label _label_8))
        (:==
          (goto _label_8))
        (:<
          (LocalVariables|Set_90or0_Z 0))))
    (:==
      (goto _label_7))
    (:<
      (Math|Integer|CompareInt (Math|Integer|%(Integer) (- _rotationindegree_6 (Math|Integer|%(Integer) _rotationindegree_3 90)) 90) -45
        (:>
          (LocalVariables|Set_Negative90or0_Z 0 :!label _label_9))
        (:==
          (goto _label_9))
        (:<
          (LocalVariables|Set_Negative90or0_Z -90)))))
  (bind _output_get_3 (LocalVariables|Set_Temp_Z (+ (LocalVariables|Get_90or0_Z) (LocalVariables|Get_Negative90or0_Z))))
  (return (Math|Conversions|ToFloat(Integer) (+ (+ _output_get (* (/ (- _rotationindegree_4 (Math|Integer|%(Integer) _rotationindegree 90)) 90) 90)) (Math|Integer|%(Integer) _rotationindegree 90))) (Math|Conversions|ToFloat(Integer) (+ (+ _output_get_2 (* (/ (- _rotationindegree_5 (Math|Integer|%(Integer) _rotationindegree_2 90)) 90) 90)) (Math|Integer|%(Integer) _rotationindegree_2 90))) (Math|Conversions|ToFloat(Integer) (+ (+ _output_get_3 (* (/ (- _rotationindegree_6 (Math|Integer|%(Integer) _rotationindegree_3 90)) 90) 90)) (Math|Integer|%(Integer) _rotationindegree_3 90)))))