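; VR wrist menu of rotating holograms for spawning grid cube pieces and marbles.
; A wrist flick, read from the Bowl's angular velocity while facing up, shows the menu until it tilts away.
; Overlapping a hologram with a motion controller's GrabCapsule highlights it and selects what to spawn, with separate marble handling.
; Pickup spawns the selection with a sound and attaches it, physics off, to the grabbing controller.
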(event OnComponentBeginOverlap(CurveCube)
  (params (OverlappedComponent :type Primitive%20Component%20Object%20Reference) (OtherActor :type Actor%20Object%20Reference) (OtherComp :type Primitive%20Component%20Object%20Reference) (OtherBodyIndex :type Integer) (bFromSweep :type Boolean) (SweepResult :type Hit%20Result%20Structure%20%28by%20ref%29))
  ;[0 0 0] Handle Hovereffect on Overlap with MotionController
  (if (CallFunction|IstheOverlappingActorMotionController? OtherActor OtherComp)
    (CallFunction|RefreshMaterials)
    (CallFunction|SetCubetoSpawn (Variables|Default|GetCurveCube) "/Game/GameElementBP/Cubes/CurveCube/BP_GridCurveCube.BP_GridCurveCube_C")))

(event OnComponentEndOverlap(CurveCube)
  (params (OverlappedComponent :type Primitive%20Component%20Object%20Reference) (OtherActor :type Actor%20Object%20Reference) (OtherComp :type Primitive%20Component%20Object%20Reference) (OtherBodyIndex :type Integer))
  ;[0 0 0] Handle Hovereffect on Overlap with MotionController
  (if (CallFunction|IstheActorThatStopsOverlappingMotionController? OtherActor OtherComp "/Game/GameElementBP/Cubes/CurveCube/BP_GridCurveCube.BP_GridCurveCube_C")
    (Variables|Default|SetObjectToSpawn 0)
    (Rendering|Material|SetMaterial (Variables|Default|GetCurveCube) 0 "/Game/GameElementBP/Material/M_Hologram_Normal.M_Hologram_Normal")))

(event OnComponentBeginOverlap(StraightHalfHoleCube)
  (params (OverlappedComponent :type Primitive%20Component%20Object%20Reference) (OtherActor :type Actor%20Object%20Reference) (OtherComp :type Primitive%20Component%20Object%20Reference) (OtherBodyIndex :type Integer) (bFromSweep :type Boolean) (SweepResult :type Hit%20Result%20Structure%20%28by%20ref%29))
  ;[0 0 0] Handle Hovereffect on Overlap with MotionController
  (if (CallFunction|IstheOverlappingActorMotionController? OtherActor OtherComp)
    (CallFunction|RefreshMaterials)
    (CallFunction|SetCubetoSpawn (Variables|Default|GetStraightHalfHoleCube) "/Game/GameElementBP/Cubes/StraightHalfHoleCube/BP_GridStraightHalfHoleCube.BP_GridStraightHalfHoleCube_C")))

(event OnComponentEndOverlap(StraightHalfHoleCube)
  (params (OverlappedComponent :type Primitive%20Component%20Object%20Reference) (OtherActor :type Actor%20Object%20Reference) (OtherComp :type Primitive%20Component%20Object%20Reference) (OtherBodyIndex :type Integer))
  ;[0 0 0] Handle Hovereffect on Overlap with MotionController
  (if (CallFunction|IstheActorThatStopsOverlappingMotionController? OtherActor OtherComp "/Game/GameElementBP/Cubes/StraightHalfHoleCube/BP_GridStraightHalfHoleCube.BP_GridStraightHalfHoleCube_C")
    (Variables|Default|SetObjectToSpawn 0)
    (Rendering|Material|SetMaterial (Variables|Default|GetStraightHalfHoleCube) 0 "/Game/GameElementBP/Material/M_Hologram_Normal.M_Hologram_Normal")))

(event OnComponentBeginOverlap(Marble)
  (params (OverlappedComponent :type Primitive%20Component%20Object%20Reference) (OtherActor :type Actor%20Object%20Reference) (OtherComp :type Primitive%20Component%20Object%20Reference) (OtherBodyIndex :type Integer) (bFromSweep :type Boolean) (SweepResult :type Hit%20Result%20Structure%20%28by%20ref%29))
  ;[0 0 0] Handle Hovereffect on Overlap with MotionController
  ;;[0 0 0] Extra handling for Marble, because it doesn't inherit GridCube.
  (if (CallFunction|IstheOverlappingActorMotionController? OtherActor OtherComp)
    (Variables|Default|SetObjectToSpawn 0)
    (Variables|Default|SetSpawnMarble? true)
    (CallFunction|RefreshMaterials)
    (Rendering|Material|SetMaterial (Variables|Default|GetMarble) 0 "/Game/GameElementBP/Material/M_Hologram_Hover.M_Hologram_Hover")))

(event OnComponentEndOverlap(Marble)
  (params (OverlappedComponent :type Primitive%20Component%20Object%20Reference) (OtherActor :type Actor%20Object%20Reference) (OtherComp :type Primitive%20Component%20Object%20Reference) (OtherBodyIndex :type Integer))
  ;[0 0 0] Handle Hovereffect on Overlap with MotionController
  ;;[0 0 0] Extra handling for Marble, because it doesn't inherit GridCube.
  (bind _asbp_motion_controller (Utilities|Casting|CastToBP_MotionController OtherActor))
  (if (and (== (Variables|/Game/VirtualRealityBP/Blueprints/BP_MotionController.BP_MotionController_C|GetGrabCapsule _asbp_motion_controller) OtherComp) (Variables|Default|GetSpawnMarble?))
    (Variables|Default|SetSpawnMarble? false)
    (Rendering|Material|SetMaterial (Variables|Default|GetMarble) 0 "/Game/GameElementBP/Material/M_Hologram_Normal.M_Hologram_Normal")))

(event OnComponentBeginOverlap(EndCube)
  (params (OverlappedComponent :type Primitive%20Component%20Object%20Reference) (OtherActor :type Actor%20Object%20Reference) (OtherComp :type Primitive%20Component%20Object%20Reference) (OtherBodyIndex :type Integer) (bFromSweep :type Boolean) (SweepResult :type Hit%20Result%20Structure%20%28by%20ref%29))
  ;[0 0 0] Handle Hovereffect on Overlap with MotionController
  (if (CallFunction|IstheOverlappingActorMotionController? OtherActor OtherComp)
    (CallFunction|RefreshMaterials)
    (CallFunction|SetCubetoSpawn (Variables|Default|GetEndCube) "/Game/GameElementBP/Cubes/EndCube/BP_GridEndCube.BP_GridEndCube_C")))

(event OnComponentEndOverlap(EndCube)
  (params (OverlappedComponent :type Primitive%20Component%20Object%20Reference) (OtherActor :type Actor%20Object%20Reference) (OtherComp :type Primitive%20Component%20Object%20Reference) (OtherBodyIndex :type Integer))
  ;[0 0 0] Handle Hovereffect on Overlap with MotionController
  (if (CallFunction|IstheActorThatStopsOverlappingMotionController? OtherActor OtherComp "/Game/GameElementBP/Cubes/EndCube/BP_GridEndCube.BP_GridEndCube_C")
    (Variables|Default|SetObjectToSpawn 0)
    (Rendering|Material|SetMaterial (Variables|Default|GetEndCube) 0 "/Game/GameElementBP/Material/M_Hologram_Normal.M_Hologram_Normal")))

(event OnComponentBeginOverlap(NormalCube)
  (params (OverlappedComponent :type Primitive%20Component%20Object%20Reference) (OtherActor :type Actor%20Object%20Reference) (OtherComp :type Primitive%20Component%20Object%20Reference) (OtherBodyIndex :type Integer) (bFromSweep :type Boolean) (SweepResult :type Hit%20Result%20Structure%20%28by%20ref%29))
  ;[0 0 0] Handle Hovereffect on Overlap with MotionController
  (if (CallFunction|IstheOverlappingActorMotionController? OtherActor OtherComp)
    (CallFunction|RefreshMaterials)
    (CallFunction|SetCubetoSpawn (Variables|Default|GetNormalCube) "/Game/GameElementBP/Cubes/NormalCube/BP_GridNormalCube.BP_GridNormalCube_C")))

(event OnComponentEndOverlap(NormalCube)
  (params (OverlappedComponent :type Primitive%20Component%20Object%20Reference) (OtherActor :type Actor%20Object%20Reference) (OtherComp :type Primitive%20Component%20Object%20Reference) (OtherBodyIndex :type Integer))
  ;[0 0 0] Handle Hovereffect on Overlap with MotionController
  (if (CallFunction|IstheActorThatStopsOverlappingMotionController? OtherActor OtherComp "/Game/GameElementBP/Cubes/NormalCube/BP_GridNormalCube.BP_GridNormalCube_C")
    (Variables|Default|SetObjectToSpawn 0)
    (Rendering|Material|SetMaterial (Variables|Default|GetNormalCube) 0 "/Game/GameElementBP/Material/M_Hologram_Normal.M_Hologram_Normal")))

(event OnComponentBeginOverlap(StraightCube)
  (params (OverlappedComponent :type Primitive%20Component%20Object%20Reference) (OtherActor :type Actor%20Object%20Reference) (OtherComp :type Primitive%20Component%20Object%20Reference) (OtherBodyIndex :type Integer) (bFromSweep :type Boolean) (SweepResult :type Hit%20Result%20Structure%20%28by%20ref%29))
  ;[0 0 0] Handle Hovereffect on Overlap with MotionController
  (if (CallFunction|IstheOverlappingActorMotionController? OtherActor OtherComp)
    (CallFunction|RefreshMaterials)
    (CallFunction|SetCubetoSpawn (Variables|Default|GetStraightCube) "/Game/GameElementBP/Cubes/StraightCube/BP_GridStraightCube.BP_GridStraightCube_C")))

(event OnComponentEndOverlap(StraightCube)
  (params (OverlappedComponent :type Primitive%20Component%20Object%20Reference) (OtherActor :type Actor%20Object%20Reference) (OtherComp :type Primitive%20Component%20Object%20Reference) (OtherBodyIndex :type Integer))
  ;[0 0 0] Handle Hovereffect on Overlap with MotionController
  (if (CallFunction|IstheActorThatStopsOverlappingMotionController? OtherActor OtherComp "/Game/GameElementBP/Cubes/StraightCube/BP_GridStraightCube.BP_GridStraightCube_C")
    (Variables|Default|SetObjectToSpawn 0)
    (Rendering|Material|SetMaterial (Variables|Default|GetStraightCube) 0 "/Game/GameElementBP/Material/M_Hologram_Normal.M_Hologram_Normal")))

(event OnComponentBeginOverlap(StraightHalfCube)
  (params (OverlappedComponent :type Primitive%20Component%20Object%20Reference) (OtherActor :type Actor%20Object%20Reference) (OtherComp :type Primitive%20Component%20Object%20Reference) (OtherBodyIndex :type Integer) (bFromSweep :type Boolean) (SweepResult :type Hit%20Result%20Structure%20%28by%20ref%29))
  ;[0 0 0] Handle Hovereffect on Overlap with MotionController
  (if (CallFunction|IstheOverlappingActorMotionController? OtherActor OtherComp)
    (CallFunction|RefreshMaterials)
    (CallFunction|SetCubetoSpawn (Variables|Default|GetStraightHalfCube) "/Game/GameElementBP/Cubes/StraightHalfCube/BP_GridStraightHalfCube.BP_GridStraightHalfCube_C")))

(event OnComponentEndOverlap(StraightHalfCube)
  (params (OverlappedComponent :type Primitive%20Component%20Object%20Reference) (OtherActor :type Actor%20Object%20Reference) (OtherComp :type Primitive%20Component%20Object%20Reference) (OtherBodyIndex :type Integer))
  ;[0 0 0] Handle Hovereffect on Overlap with MotionController
  (if (CallFunction|IstheActorThatStopsOverlappingMotionController? OtherActor OtherComp "/Game/GameElementBP/Cubes/StraightHalfCube/BP_GridStraightHalfCube.BP_GridStraightHalfCube_C")
    (Variables|Default|SetObjectToSpawn 0)
    (Rendering|Material|SetMaterial (Variables|Default|GetStraightHalfCube) 0 "/Game/GameElementBP/Material/M_Hologram_Normal.M_Hologram_Normal")))

(event EventTick
  (params (DeltaSeconds :type Float%20%28single-precision%29))
  ;[0 0 0] Handles the visibility and rotation of the BlockMenu.
  (if (CallFunction|DidWristGotFlickedUp?)
    (Variables|Default|SetIsVisible true))
  (if (and (Variables|Default|GetIsVisible) (not (CallFunction|IsUpVectorShowingUp (Variables|Default|GetUp%20Threshold))))
    (Variables|Default|SetIsVisible false))
  (if (Variables|Default|GetIsVisible)
    (CallFunction|RotateAllObjects)
    (Utilities|FlowControl|DoOnce false :!label _label
      (:Completed
        (CallFunction|SetMeshVisibility true)
        (CallFunction|SetCollisionOfAllObjects true)
        (goto _label_2 Reset)))
    (else
      (Utilities|FlowControl|DoOnce false :!label _label_2
        (:Completed
          (CallFunction|SetMeshVisibility false)
          (CallFunction|SetCollisionOfAllObjects false)
          (goto _label Reset))))))

(event EventPickup
  (params (AttachTo :type Scene%20Component%20Object%20Reference))
  (bind _returnvalue (Transformation|GetActorLocation))
  (bind _returnvalue_2 (Math|Transform|MakeTransform _returnvalue))
  ;[0 0 0] SpawnObjects
  (bind _asbp_motion_controller (Utilities|Casting|CastToBP_MotionController (Components|GetOwner AttachTo)))
  (Variables|Default|SetMotion%20Controller _asbp_motion_controller)
  (if (Variables|Default|GetSpawnMarble?)
    ;;[0 0 0] SpawnMarble
    (bind _returnvalue_3 (Game|SpawnActorfromClass "/Game/GameElementBP/BP_Marble.BP_Marble_C" _returnvalue_2 "Undefined" self 0))
    (Audio|PlaySoundatLocation "/Game/Audio/FXPack/inverted_spawn_Cue.inverted_spawn_Cue" _returnvalue "0, 0, 0" 1.0 1.0 0.0 0 0 0)
    (Utilities|Set|Add (Variables|/Game/VirtualRealityBP/Blueprints/BP_MotionController.BP_MotionController_C|GetAttachedActors (Variables|Default|GetMotion%20Controller)) _returnvalue_3)
    (Physics|SetSimulatePhysics (Variables|/Script/Engine.StaticMeshActor|GetStaticMeshComponent _returnvalue_3) false)
    (Transformation|AttachComponentToComponent (Variables|/Script/Engine.StaticMeshActor|GetStaticMeshComponent _returnvalue_3) AttachTo "None" "SnapToTarget" "KeepWorld" "KeepWorld" false)
    (Variables|/Game/GameElementBP/BP_Marble.BP_Marble_C|SetIsGrabbed _returnvalue_3 true)
    (else
      (bind _objecttospawn (Variables|Default|GetObjectToSpawn)
        (:then
          ;;[0 0 0] SpawnCube
          (bind _returnvalue_4 (Game|SpawnActorfromClass _objecttospawn _returnvalue_2 "Undefined" self 0))
          (Audio|PlaySoundatLocation "/Game/Audio/FXPack/inverted_spawn_Cue.inverted_spawn_Cue" _returnvalue "0, 0, 0" 1.0 1.0 0.0 0 0 0)
          (Utilities|Set|Add (Variables|/Game/VirtualRealityBP/Blueprints/BP_MotionController.BP_MotionController_C|GetAttachedActors (Variables|Default|GetMotion%20Controller)) _returnvalue_4)
          (Physics|SetSimulatePhysics (Variables|/Script/Engine.StaticMeshActor|GetStaticMeshComponent _returnvalue_4) false)
          (Transformation|AttachComponentToComponent (Variables|/Script/Engine.StaticMeshActor|GetStaticMeshComponent _returnvalue_4) AttachTo "None" "SnapToTarget" "KeepWorld" "KeepWorld" false)
          (Variables|/Game/GameElementBP/BP_GridCube.BP_GridCube_C|SetIsGrabbed _returnvalue_4 true))
        (:else)))))

(fn ConstructionScript)

(fn RotateAllObjects
  (Transformation|AddLocalRotation (Variables|Default|GetCurveCube) "1.000000,1.000000,0.000000" false false))

(fn IsUpVectorShowingUp
  (params (UpThreshold :type Float%20%28single-precision%29))
  (bind _returnvalue (Transformation|GetActorRotation))
  (bind _z_axis (LocalVariables|GetZ-Axis))
  (bind _returnvalue_2 (Math|Vector|GetUpVector _returnvalue))
  (return (> (Class|KismetMathLibrary|DegAsin (/ (Math|Vector|DotProduct _z_axis _returnvalue_2) (* (Math|Vector|VectorLength _returnvalue_2) (Math|Vector|VectorLength _z_axis)))) UpThreshold)))

(fn SetMeshVisibility
  (params (IsVisible :type Boolean))
  (Rendering|SetVisibility (Variables|Default|GetCurveCube) IsVisible false))

(fn RefreshMaterials
  (Rendering|Material|SetMaterial (Variables|Default|GetCurveCube) 0 "/Game/GameElementBP/Material/M_Hologram_Normal.M_Hologram_Normal"))

(fn SetCollisionOfAllObjects
  (params (EnableCollision :type Boolean))
  (bind _curvecube (Variables|Default|GetCurveCube))
  (if EnableCollision
    (Collision|SetCollisionEnabled _curvecube "QueryOnly")
    (else
      (Collision|SetCollisionEnabled _curvecube "NoCollision"))))

(fn IsAngularVelocityOverThreshold
  (params (VelocityThreshold :type Float%20%28single-precision%29))
  (bind _bowl (Variables|Default|GetBowl))
  (bind _returnvalue (Physics|GetPhysicsAngularVelocityinDegrees _bowl "None"))
  (return (or (>= (Math|Float|Absolute(Float) (.x _returnvalue)) VelocityThreshold) (>= (Math|Float|Absolute(Float) (.y _returnvalue)) VelocityThreshold))))

(fn IstheOverlappingActorMotionController?
  (params (OtherActor :type Object%20Object%20Reference) (OtherComp :type Object%20Object%20Reference))
  (if (Rendering|IsVisible (Variables|Default|GetCurveCube))
    (bind _asbp_motion_controller (Utilities|Casting|CastToBP_MotionController OtherActor))
    (return (== (Variables|/Game/VirtualRealityBP/Blueprints/BP_MotionController.BP_MotionController_C|GetGrabCapsule _asbp_motion_controller) OtherComp))))

(fn SetCubetoSpawn
  (params (Hologramm :type Primitive%20Component%20Object%20Reference) (ObjectClass :type BP%20Grid%20Cube%20Class%20Reference))
  (Rendering|Material|SetMaterial Hologramm 0 "/Game/GameElementBP/Material/M_Hologram_Hover.M_Hologram_Hover")
  (Variables|Default|SetObjectToSpawn ObjectClass)
  (Variables|Default|SetSpawnMarble? false))

(fn IstheActorThatStopsOverlappingMotionController?
  (params (OtherActor :type Object%20Object%20Reference) (OtherComp :type Object%20Object%20Reference) (ObjectThatStopsToOverlap :type BP%20Grid%20Cube%20Class%20Reference))
  (bind _asbp_motion_controller (Utilities|Casting|CastToBP_MotionController OtherActor))
  (return (and (== (Variables|/Game/VirtualRealityBP/Blueprints/BP_MotionController.BP_MotionController_C|GetGrabCapsule _asbp_motion_controller) OtherComp) (== (Variables|Default|GetObjectToSpawn) ObjectThatStopsToOverlap))))

(fn DidWristGotFlickedUp?
  (return (and (CallFunction|IsAngularVelocityOverThreshold (Variables|Default|GetVelocity%20Threshold)) (CallFunction|IsUpVectorShowingUp (Variables|Default|GetUp%20Threshold)))))