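; VR hologram menu for picking marble-track grid blocks or a marble with a motion controller.
; While in use, Tick spins the items and toggles their visibility and collision based on whether the menu's up vector points upward.
; Grab-sphere overlaps set the selected item and highlight it red.
; Pickup spawns that selection and attaches it to the given controller component with physics off.
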(event OnComponentBeginOverlap(CurveCube)
  (params (OverlappedComponent :type Primitive%20Component%20Object%20Reference) (OtherActor :type Actor%20Object%20Reference) (OtherComp :type Primitive%20Component%20Object%20Reference) (OtherBodyIndex :type Integer) (bFromSweep :type Boolean) (SweepResult :type Hit%20Result%20Structure%20%28by%20ref%29))
  (if (Rendering|IsVisible (Variables|Default|GetCurveCube))
    (bind _asbp_motion_controller (Utilities|Casting|CastToBP_MotionController OtherActor))
    (if (== (Variables|/Game/VirtualRealityBP/Blueprints/BP_MotionController.BP_MotionController_C|GetGrabSphere _asbp_motion_controller) OtherComp)
      (Variables|Default|SetObjectToSpawn "/Game/GameElementBP/Cubes/CurveCube/BP_GridCurveCube.BP_GridCurveCube_C")
      (Variables|Default|SetSpawnMarble? false)
      (CallFunction|RefreshMaterials)
      (Rendering|Material|SetMaterial (Variables|Default|GetCurveCube) 0 "/Game/GameElementBP/Material/M_Hologram_Red.M_Hologram_Red"))))

(event OnComponentEndOverlap(CurveCube)
  (params (OverlappedComponent :type Primitive%20Component%20Object%20Reference) (OtherActor :type Actor%20Object%20Reference) (OtherComp :type Primitive%20Component%20Object%20Reference) (OtherBodyIndex :type Integer))
  (bind _asbp_motion_controller (Utilities|Casting|CastToBP_MotionController OtherActor))
  (if (and (== (Variables|/Game/VirtualRealityBP/Blueprints/BP_MotionController.BP_MotionController_C|GetGrabSphere _asbp_motion_controller) OtherComp) (== (Variables|Default|GetObjectToSpawn) "/Game/GameElementBP/Cubes/CurveCube/BP_GridCurveCube.BP_GridCurveCube_C"))
    (Variables|Default|SetObjectToSpawn 0)
    (Rendering|Material|SetMaterial (Variables|Default|GetCurveCube) 0 "/Game/GameElementBP/Material/M_Hologram_Blue.M_Hologram_Blue")))

(event OnComponentBeginOverlap(StraightHalfHoleCube)
  (params (OverlappedComponent :type Primitive%20Component%20Object%20Reference) (OtherActor :type Actor%20Object%20Reference) (OtherComp :type Primitive%20Component%20Object%20Reference) (OtherBodyIndex :type Integer) (bFromSweep :type Boolean) (SweepResult :type Hit%20Result%20Structure%20%28by%20ref%29))
  (if (Rendering|IsVisible (Variables|Default|GetCurveCube))
    (bind _asbp_motion_controller (Utilities|Casting|CastToBP_MotionController OtherActor))
    (if (== (Variables|/Game/VirtualRealityBP/Blueprints/BP_MotionController.BP_MotionController_C|GetGrabSphere _asbp_motion_controller) OtherComp)
      (Variables|Default|SetObjectToSpawn "/Game/GameElementBP/Cubes/StraightHalfHoleCube/BP_GridStraightHalfHoleCube.BP_GridStraightHalfHoleCube_C")
      (Variables|Default|SetSpawnMarble? false)
      (CallFunction|RefreshMaterials)
      (Rendering|Material|SetMaterial (Variables|Default|GetStraightHalfHoleCube) 0 "/Game/GameElementBP/Material/M_Hologram_Red.M_Hologram_Red"))))

(event OnComponentEndOverlap(StraightHalfHoleCube)
  (params (OverlappedComponent :type Primitive%20Component%20Object%20Reference) (OtherActor :type Actor%20Object%20Reference) (OtherComp :type Primitive%20Component%20Object%20Reference) (OtherBodyIndex :type Integer))
  (bind _asbp_motion_controller (Utilities|Casting|CastToBP_MotionController OtherActor))
  (if (and (== (Variables|/Game/VirtualRealityBP/Blueprints/BP_MotionController.BP_MotionController_C|GetGrabSphere _asbp_motion_controller) OtherComp) (== (Variables|Default|GetObjectToSpawn) "/Game/GameElementBP/Cubes/StraightHalfHoleCube/BP_GridStraightHalfHoleCube.BP_GridStraightHalfHoleCube_C"))
    (Variables|Default|SetObjectToSpawn 0)
    (Rendering|Material|SetMaterial (Variables|Default|GetStraightHalfHoleCube) 0 "/Game/GameElementBP/Material/M_Hologram_Blue.M_Hologram_Blue")))

(event OnComponentBeginOverlap(Marble)
  (params (OverlappedComponent :type Primitive%20Component%20Object%20Reference) (OtherActor :type Actor%20Object%20Reference) (OtherComp :type Primitive%20Component%20Object%20Reference) (OtherBodyIndex :type Integer) (bFromSweep :type Boolean) (SweepResult :type Hit%20Result%20Structure%20%28by%20ref%29))
  (if (Rendering|IsVisible (Variables|Default|GetCurveCube))
    (bind _asbp_motion_controller (Utilities|Casting|CastToBP_MotionController OtherActor))
    (if (== (Variables|/Game/VirtualRealityBP/Blueprints/BP_MotionController.BP_MotionController_C|GetGrabSphere _asbp_motion_controller) OtherComp)
      (Variables|Default|SetObjectToSpawn 0)
      (Variables|Default|SetSpawnMarble? true)
      (CallFunction|RefreshMaterials)
      (Rendering|Material|SetMaterial (Variables|Default|GetMarble) 0 "/Game/GameElementBP/Material/M_Hologram_Red.M_Hologram_Red"))))

(event OnComponentEndOverlap(Marble)
  (params (OverlappedComponent :type Primitive%20Component%20Object%20Reference) (OtherActor :type Actor%20Object%20Reference) (OtherComp :type Primitive%20Component%20Object%20Reference) (OtherBodyIndex :type Integer))
  (bind _asbp_motion_controller (Utilities|Casting|CastToBP_MotionController OtherActor))
  (if (and (== (Variables|/Game/VirtualRealityBP/Blueprints/BP_MotionController.BP_MotionController_C|GetGrabSphere _asbp_motion_controller) OtherComp) (Variables|Default|GetSpawnMarble?))
    (Variables|Default|SetSpawnMarble? false)
    (Rendering|Material|SetMaterial (Variables|Default|GetMarble) 0 "/Game/GameElementBP/Material/M_Hologram_Blue.M_Hologram_Blue")))

(event OnComponentBeginOverlap(EndCube)
  (params (OverlappedComponent :type Primitive%20Component%20Object%20Reference) (OtherActor :type Actor%20Object%20Reference) (OtherComp :type Primitive%20Component%20Object%20Reference) (OtherBodyIndex :type Integer) (bFromSweep :type Boolean) (SweepResult :type Hit%20Result%20Structure%20%28by%20ref%29))
  (if (Rendering|IsVisible (Variables|Default|GetCurveCube))
    (bind _asbp_motion_controller (Utilities|Casting|CastToBP_MotionController OtherActor))
    (if (== (Variables|/Game/VirtualRealityBP/Blueprints/BP_MotionController.BP_MotionController_C|GetGrabSphere _asbp_motion_controller) OtherComp)
      (Variables|Default|SetObjectToSpawn "/Game/GameElementBP/Cubes/EndCube/BP_GridEndCube.BP_GridEndCube_C")
      (Variables|Default|SetSpawnMarble? false)
      (CallFunction|RefreshMaterials)
      (Rendering|Material|SetMaterial (Variables|Default|GetEndCube) 0 "/Game/GameElementBP/Material/M_Hologram_Red.M_Hologram_Red"))))

(event OnComponentEndOverlap(EndCube)
  (params (OverlappedComponent :type Primitive%20Component%20Object%20Reference) (OtherActor :type Actor%20Object%20Reference) (OtherComp :type Primitive%20Component%20Object%20Reference) (OtherBodyIndex :type Integer))
  (bind _asbp_motion_controller (Utilities|Casting|CastToBP_MotionController OtherActor))
  (if (and (== (Variables|/Game/VirtualRealityBP/Blueprints/BP_MotionController.BP_MotionController_C|GetGrabSphere _asbp_motion_controller) OtherComp) (== (Variables|Default|GetObjectToSpawn) "/Game/GameElementBP/Cubes/EndCube/BP_GridEndCube.BP_GridEndCube_C"))
    (Variables|Default|SetObjectToSpawn 0)
    (Rendering|Material|SetMaterial (Variables|Default|GetEndCube) 0 "/Game/GameElementBP/Material/M_Hologram_Blue.M_Hologram_Blue")))

(event OnComponentBeginOverlap(NormalCube)
  (params (OverlappedComponent :type Primitive%20Component%20Object%20Reference) (OtherActor :type Actor%20Object%20Reference) (OtherComp :type Primitive%20Component%20Object%20Reference) (OtherBodyIndex :type Integer) (bFromSweep :type Boolean) (SweepResult :type Hit%20Result%20Structure%20%28by%20ref%29))
  (if (Rendering|IsVisible (Variables|Default|GetCurveCube))
    (bind _asbp_motion_controller (Utilities|Casting|CastToBP_MotionController OtherActor))
    (if (== (Variables|/Game/VirtualRealityBP/Blueprints/BP_MotionController.BP_MotionController_C|GetGrabSphere _asbp_motion_controller) OtherComp)
      (Variables|Default|SetObjectToSpawn "/Game/GameElementBP/Cubes/NormalCube/BP_GridNormalCube.BP_GridNormalCube_C")
      (Variables|Default|SetSpawnMarble? false)
      (CallFunction|RefreshMaterials)
      (Rendering|Material|SetMaterial (Variables|Default|GetNormalCube) 0 "/Game/GameElementBP/Material/M_Hologram_Red.M_Hologram_Red"))))

(event OnComponentEndOverlap(NormalCube)
  (params (OverlappedComponent :type Primitive%20Component%20Object%20Reference) (OtherActor :type Actor%20Object%20Reference) (OtherComp :type Primitive%20Component%20Object%20Reference) (OtherBodyIndex :type Integer))
  (bind _asbp_motion_controller (Utilities|Casting|CastToBP_MotionController OtherActor))
  (if (and (== (Variables|/Game/VirtualRealityBP/Blueprints/BP_MotionController.BP_MotionController_C|GetGrabSphere _asbp_motion_controller) OtherComp) (== (Variables|Default|GetObjectToSpawn) "/Game/GameElementBP/Cubes/NormalCube/BP_GridNormalCube.BP_GridNormalCube_C"))
    (Variables|Default|SetObjectToSpawn 0)
    (Rendering|Material|SetMaterial (Variables|Default|GetNormalCube) 0 "/Game/GameElementBP/Material/M_Hologram_Blue.M_Hologram_Blue")))

(event OnComponentBeginOverlap(StraightCube)
  (params (OverlappedComponent :type Primitive%20Component%20Object%20Reference) (OtherActor :type Actor%20Object%20Reference) (OtherComp :type Primitive%20Component%20Object%20Reference) (OtherBodyIndex :type Integer) (bFromSweep :type Boolean) (SweepResult :type Hit%20Result%20Structure%20%28by%20ref%29))
  (if (Rendering|IsVisible (Variables|Default|GetCurveCube))
    (bind _asbp_motion_controller (Utilities|Casting|CastToBP_MotionController OtherActor))
    (if (== (Variables|/Game/VirtualRealityBP/Blueprints/BP_MotionController.BP_MotionController_C|GetGrabSphere _asbp_motion_controller) OtherComp)
      (Variables|Default|SetObjectToSpawn "/Game/GameElementBP/Cubes/StraightCube/BP_GridStraightCube.BP_GridStraightCube_C")
      (Variables|Default|SetSpawnMarble? false)
      (CallFunction|RefreshMaterials)
      (Rendering|Material|SetMaterial (Variables|Default|GetStraightCube) 0 "/Game/GameElementBP/Material/M_Hologram_Red.M_Hologram_Red"))))

(event OnComponentEndOverlap(StraightCube)
  (params (OverlappedComponent :type Primitive%20Component%20Object%20Reference) (OtherActor :type Actor%20Object%20Reference) (OtherComp :type Primitive%20Component%20Object%20Reference) (OtherBodyIndex :type Integer))
  (bind _asbp_motion_controller (Utilities|Casting|CastToBP_MotionController OtherActor))
  (if (and (== (Variables|/Game/VirtualRealityBP/Blueprints/BP_MotionController.BP_MotionController_C|GetGrabSphere _asbp_motion_controller) OtherComp) (== (Variables|Default|GetObjectToSpawn) "/Game/GameElementBP/Cubes/StraightCube/BP_GridStraightCube.BP_GridStraightCube_C"))
    (Variables|Default|SetObjectToSpawn 0)
    (Rendering|Material|SetMaterial (Variables|Default|GetStraightCube) 0 "/Game/GameElementBP/Material/M_Hologram_Blue.M_Hologram_Blue")))

(event OnComponentBeginOverlap(StraightHalfCube)
  (params (OverlappedComponent :type Primitive%20Component%20Object%20Reference) (OtherActor :type Actor%20Object%20Reference) (OtherComp :type Primitive%20Component%20Object%20Reference) (OtherBodyIndex :type Integer) (bFromSweep :type Boolean) (SweepResult :type Hit%20Result%20Structure%20%28by%20ref%29))
  (if (Rendering|IsVisible (Variables|Default|GetCurveCube))
    (bind _asbp_motion_controller (Utilities|Casting|CastToBP_MotionController OtherActor))
    (if (== (Variables|/Game/VirtualRealityBP/Blueprints/BP_MotionController.BP_MotionController_C|GetGrabSphere _asbp_motion_controller) OtherComp)
      (Variables|Default|SetObjectToSpawn "/Game/GameElementBP/Cubes/StraightHalfCube/BP_GridStraightHalfCube.BP_GridStraightHalfCube_C")
      (Variables|Default|SetSpawnMarble? false)
      (CallFunction|RefreshMaterials)
      (Rendering|Material|SetMaterial (Variables|Default|GetStraightHalfCube) 0 "/Game/GameElementBP/Material/M_Hologram_Red.M_Hologram_Red"))))

(event OnComponentEndOverlap(StraightHalfCube)
  (params (OverlappedComponent :type Primitive%20Component%20Object%20Reference) (OtherActor :type Actor%20Object%20Reference) (OtherComp :type Primitive%20Component%20Object%20Reference) (OtherBodyIndex :type Integer))
  (bind _asbp_motion_controller (Utilities|Casting|CastToBP_MotionController OtherActor))
  (if (and (== (Variables|/Game/VirtualRealityBP/Blueprints/BP_MotionController.BP_MotionController_C|GetGrabSphere _asbp_motion_controller) OtherComp) (== (Variables|Default|GetObjectToSpawn) "/Game/GameElementBP/Cubes/StraightHalfCube/BP_GridStraightHalfCube.BP_GridStraightHalfCube_C"))
    (Variables|Default|SetObjectToSpawn 0)
    (Rendering|Material|SetMaterial (Variables|Default|GetStraightHalfCube) 0 "/Game/GameElementBP/Material/M_Hologram_Blue.M_Hologram_Blue")))

(event EventTick
  (params (DeltaSeconds :type Float%20%28single-precision%29))
  (if (Variables|Default|GetInUse)
    (Utilities|FlowControl|Sequence
      (:then_0
        (Utilities|FlowControl|DoOnce false :!label _label
          (:Completed
            (CallFunction|SetMeshVisibility true)
            (CallFunction|SetCollisionOfAllObjects true)
            (goto _label_4 Reset))))
      (:then_1
        (if (CallFunction|IsUpVectorShowingUp)
          (CallFunction|RotateAllObjects)
          (Utilities|FlowControl|DoOnce false :!label _label_2
            (:Completed
              (CallFunction|SetMeshVisibility true)
              (CallFunction|SetCollisionOfAllObjects true)
              (goto _label_3 Reset)))
          (else
            (Utilities|FlowControl|DoOnce false :!label _label_3
              (:Completed
                (CallFunction|SetMeshVisibility false)
                (CallFunction|SetCollisionOfAllObjects false)
                (goto _label_2 Reset)))))))
    (else
      (Utilities|FlowControl|DoOnce false :!label _label_4
        (:Completed
          (CallFunction|SetMeshVisibility false)
          (CallFunction|SetCollisionOfAllObjects false)
          (goto _label Reset))))))

(event EventPickup
  (params (AttachTo :type Scene%20Component%20Object%20Reference))
  (bind _returnvalue (Transformation|GetWorldLocation AttachTo))
  (bind _returnvalue_2 (Math|Transform|MakeTransform _returnvalue))
  (bind _asbp_motion_controller (Utilities|Casting|CastToBP_MotionController (Components|GetOwner AttachTo)))
  (if (Variables|Default|GetSpawnMarble?)
    (bind _returnvalue_3 (Game|SpawnActorfromClass "/Game/GameElementBP/BP_Marble.BP_Marble_C" _returnvalue_2 "Undefined" 0 0))
    (Variables|/Game/VirtualRealityBP/Blueprints/BP_MotionController.BP_MotionController_C|SetAttachedActor _asbp_motion_controller _returnvalue_3)
    (Physics|SetSimulatePhysics (Variables|/Script/Engine.StaticMeshActor|GetStaticMeshComponent _returnvalue_3) false)
    (Transformation|AttachComponentToComponent (Variables|/Script/Engine.StaticMeshActor|GetStaticMeshComponent _returnvalue_3) AttachTo "None" "SnapToTarget" "KeepWorld" "KeepWorld" false)
    (else
      (bind _objecttospawn (Variables|Default|GetObjectToSpawn)
        (:then
          (bind _returnvalue_4 (Game|SpawnActorfromClass _objecttospawn _returnvalue_2 "Undefined" 0 0))
          (Variables|/Game/VirtualRealityBP/Blueprints/BP_MotionController.BP_MotionController_C|SetAttachedActor _asbp_motion_controller _returnvalue_4)
          (Physics|SetSimulatePhysics (Variables|/Script/Engine.StaticMeshActor|GetStaticMeshComponent _returnvalue_4) false)
          (Transformation|AttachComponentToComponent (Variables|/Script/Engine.StaticMeshActor|GetStaticMeshComponent _returnvalue_4) AttachTo "None" "SnapToTarget" "KeepWorld" "KeepWorld" false)
          (Class|PrimitiveComponent|SetConstraintMode (Variables|/Script/Engine.StaticMeshActor|GetStaticMeshComponent _returnvalue_4) "None")
          (Actor|Tick|SetActorTickEnabled _returnvalue_4 true)
          (Variables|/Game/GameElementBP/BP_GridCube.BP_GridCube_C|SetIsGrabbed _returnvalue_4 true))
        (:else)))))

(fn ConstructionScript)

(fn RotateAllObjects
  (Transformation|AddLocalRotation (Variables|Default|GetCurveCube) "2.000000,2.000000,0.000000" false false))

(fn IsUpVectorShowingUp
  (bind _returnvalue (Transformation|GetActorRotation))
  (bind _z_axis (LocalVariables|GetZ-Axis))
  (bind _returnvalue_2 (Math|Vector|GetUpVector _returnvalue))
  (return (> (Class|KismetMathLibrary|DegAsin (/ (Math|Vector|DotProduct _z_axis _returnvalue_2) (* (Math|Vector|VectorLength _returnvalue_2) (Math|Vector|VectorLength _z_axis)))) 6e+01)))

(fn SetMeshVisibility
  (params (IsVisible :type Boolean))
  (Rendering|SetVisibility (Variables|Default|GetCurveCube) IsVisible false))

(fn RefreshMaterials
  (Rendering|Material|SetMaterial (Variables|Default|GetCurveCube) 0 "/Game/GameElementBP/Material/M_Hologram_Blue.M_Hologram_Blue")
  (Rendering|Material|SetMaterial (Variables|Default|GetEndCube) 0 "/Game/GameElementBP/Material/M_Hologram_Blue.M_Hologram_Blue")
  (Rendering|Material|SetMaterial (Variables|Default|GetNormalCube) 0 "/Game/GameElementBP/Material/M_Hologram_Blue.M_Hologram_Blue")
  (Rendering|Material|SetMaterial (Variables|Default|GetStraightCube) 0 "/Game/GameElementBP/Material/M_Hologram_Blue.M_Hologram_Blue")
  (Rendering|Material|SetMaterial (Variables|Default|GetStraightHalfCube) 0 "/Game/GameElementBP/Material/M_Hologram_Blue.M_Hologram_Blue")
  (Rendering|Material|SetMaterial (Variables|Default|GetStraightHalfHoleCube) 0 "/Game/GameElementBP/Material/M_Hologram_Blue.M_Hologram_Blue")
  (Rendering|Material|SetMaterial (Variables|Default|GetMarble) 0 "/Game/GameElementBP/Material/M_Hologram_Blue.M_Hologram_Blue"))

(fn SetCollisionOfAllObjects
  (params (EnableCollision :type Boolean))
  (bind _curvecube (Variables|Default|GetCurveCube))
  (if EnableCollision
    (Collision|SetCollisionEnabled _curvecube "QueryOnly")
    (else
      (Collision|SetCollisionEnabled _curvecube "NoCollision"))))