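; VR wrist slot, used as a child actor, that stores one BP_PickupCube held by the opposite hand.
; Its sphere binds the cube's pickup/drop events; on drop, a timeline lerps it into place, then attaches it with pickup and collision disabled.
; A controller's GrabSphere overlap re-enables both and starts Tick, which interpolates the cube toward its AttachToComp.
; Leaving snaps it back; pickup stops Tick and frees the slot.
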(event OnComponentBeginOverlap(Sphere)
  (params (OverlappedComponent :type Primitive%20Component%20Object%20Reference) (OtherActor :type Actor%20Object%20Reference) (OtherComp :type Primitive%20Component%20Object%20Reference) (OtherBodyIndex :type Integer) (bFromSweep :type Boolean) (SweepResult :type Hit%20Result%20Structure%20%28by%20ref%29))
  (if (not (Variables|Default|GetIsSlotUsed))
    (bind _asbp_pickup_cube (Utilities|Casting|CastToBP_PickupCube OtherActor))
    (if (== (Variables|/Script/Engine.StaticMeshActor|GetStaticMeshComponent _asbp_pickup_cube) OtherComp)
      (Variables|Default|SetShouldStoreItem true)
      (Variables|Default|SetItemToStore _asbp_pickup_cube)
      (if (CallFunction|IsWristSlotonOtherHand)
        (EventDispatchers|BindEventtoOnPickup (Variables|Default|GetItemToStore) (EventDispatchers|CreateEvent :!event Custom|OnItemStoredPickedUp))
        (EventDispatchers|BindEventtoOnDrop (Variables|Default|GetItemToStore) (EventDispatchers|CreateEvent :!event Custom|OnItemStoredDropped))))
    (else
      (bind _asbp_motion_controller (Utilities|Casting|CastToBP_MotionController OtherActor))
      (if (== (Variables|/Game/VirtualRealityBP/Blueprints/BP_MotionController.BP_MotionController_C|GetGrabSphere _asbp_motion_controller) OtherComp)
        (Actor|Tick|SetActorTickEnabled true)
        (bind _itemtostore (Variables|Default|GetItemToStore)
          (:then
            (Variables|/Game/GameElementBP/BP_PickupCube.BP_PickupCube_C|SetCanPickUpItem _itemtostore true)
            (Collision|SetActorEnableCollision (Variables|Default|GetItemToStore) true))
          (:else))))))

(event OnComponentEndOverlap(Sphere)
  (params (OverlappedComponent :type Primitive%20Component%20Object%20Reference) (OtherActor :type Actor%20Object%20Reference) (OtherComp :type Primitive%20Component%20Object%20Reference) (OtherBodyIndex :type Integer))
  (if (not (Variables|Default|GetIsSlotUsed))
    (bind _asbp_pickup_cube (Utilities|Casting|CastToBP_PickupCube OtherActor))
    (if (== (Variables|/Script/Engine.StaticMeshActor|GetStaticMeshComponent _asbp_pickup_cube) OtherComp)
      (bind _itemtostore (Variables|Default|GetItemToStore)
        (:then
          (if (not (Variables|/Game/GameElementBP/BP_PickupCube.BP_PickupCube_C|GetIsPickedUp _itemtostore))
            (CallFunction|ResetState)))
        (:else)))
    (else
      (bind _asbp_motion_controller (Utilities|Casting|CastToBP_MotionController OtherActor))
      (if (== (Variables|/Game/VirtualRealityBP/Blueprints/BP_MotionController.BP_MotionController_C|GetGrabSphere _asbp_motion_controller) OtherComp)
        (Actor|Tick|SetActorTickEnabled false)
        (CallFunction|ObjecttoSlot)
        (bind _itemtostore_2 (Variables|Default|GetItemToStore)
          (:then
            (Variables|/Game/GameElementBP/BP_PickupCube.BP_PickupCube_C|SetCanPickUpItem _itemtostore_2 false)
            (Collision|SetActorEnableCollision (Variables|Default|GetItemToStore) false))
          (:else))))))

(event Custom|OnItemStoredPickedUp
  (Variables|Default|GetItemToStore
    (:then
      (if (Class|Actor|IsActorTickEnabled)
        (Actor|Tick|SetActorTickEnabled false)
        (Variables|/Game/GameElementBP/BP_PickupCube.BP_PickupCube_C|SetIsInWrist (Variables|Default|GetItemToStore) false)
        (CallFunction|ResetState)))
    (:else)))

(event Custom|OnItemStoredDropped
  (bind _itemtostore (Variables|Default|GetItemToStore))
  (if (Variables|Default|GetShouldStoreItem)
    (Variables|Default|SetIsSlotUsed true)
    (Variables|Default|GetItemToStore
      (:then
        (if (CallFunction|IsWristSlotonOtherHand)
          (Physics|SetSimulatePhysics (Variables|/Script/Engine.StaticMeshActor|GetStaticMeshComponent (Variables|Default|GetItemToStore)) false)
          (Variables|Default|SetItemInitTransform (Transformation|GetActorTransform (Variables|Default|GetItemToStore)))
          (Components|Timeline|SetPlayRate (Variables|Default|GetSnapToWrist) (/ 1.0 (Variables|Default|GetAnimationSpeed)))
          (bind _alpha (Timeline|SnapToWrist PlayFromStart)
            (:Update
              (Transformation|SetActorTransform (Variables|Default|GetItemToStore) (Math|Transform|Lerp(Transform) (Variables|Default|GetItemInitTransform) (Transformation|GetWorldTransform (Variables|Default|GetItemLocation)) _alpha)))
            (:Finished
              (Transformation|AttachComponentToComponent (Variables|Default|GetItemToStore) (Variables|Transformation|GetRootComponent) "None" "KeepWorld" "KeepWorld" "KeepRelative" true)
              (Variables|/Game/GameElementBP/BP_PickupCube.BP_PickupCube_C|SetCanPickUpItem _itemtostore false)
              (Variables|/Game/GameElementBP/BP_PickupCube.BP_PickupCube_C|SetIsInWrist _itemtostore true)
              (Collision|SetActorEnableCollision (Variables|Default|GetItemToStore) false)))))
      (:else))))

(event Custom|ObjectToSlot
  (bind _itemtostore (Variables|Default|GetItemToStore))
  (Variables|Default|SetItemInitTransform (Transformation|GetActorTransform (Variables|Default|GetItemToStore)))
  (Components|Timeline|SetPlayRate (Variables|Default|GetSnapToWrist) (/ 1.0 (Variables|Default|GetAnimationSpeed)))
  (bind _alpha (Timeline|SnapToWrist PlayFromStart)
    (:Update
      (Transformation|SetActorTransform (Variables|Default|GetItemToStore) (Math|Transform|Lerp(Transform) (Variables|Default|GetItemInitTransform) (Transformation|GetWorldTransform (Variables|Default|GetItemLocation)) _alpha)))
    (:Finished
      (Transformation|AttachComponentToComponent (Variables|Default|GetItemToStore) (Variables|Transformation|GetRootComponent) "None" "KeepWorld" "KeepWorld" "KeepRelative" true)
      (Variables|/Game/GameElementBP/BP_PickupCube.BP_PickupCube_C|SetCanPickUpItem _itemtostore false)
      (Variables|/Game/GameElementBP/BP_PickupCube.BP_PickupCube_C|SetIsInWrist _itemtostore true)
      (Collision|SetActorEnableCollision (Variables|Default|GetItemToStore) false))))

(event EventTick
  (params (DeltaSeconds :type Float%20%28single-precision%29))
  (bind _itemtostore (Variables|Default|GetItemToStore)
    (:then
      (Variables|/Game/GameElementBP/BP_PickupCube.BP_PickupCube_C|GetAttachToComp _itemtostore
        (:then
          (Transformation|SetActorTransform (Variables|Default|GetItemToStore) (CallFunction|GetObjectTransform)))
        (:else)))
    (:else)))

(fn ConstructionScript)

(fn IsWristSlotonOtherHand
  (bind _itemtostore (Variables|Default|GetItemToStore)
    (:then
      (Utilities|IsValid (Variables|/Game/GameElementBP/BP_PickupCube.BP_PickupCube_C|GetAttachToComp _itemtostore)
        (:Is%20Valid
          (return (and (!= (Components|GetOwner (Variables|/Game/GameElementBP/BP_PickupCube.BP_PickupCube_C|GetAttachToComp _itemtostore)) (Actor|GetParentActor)) (Variables|/Game/GameElementBP/BP_PickupCube.BP_PickupCube_C|GetIsPickedUp _itemtostore))))
        (:Is%20Not%20Valid
          _)))
    (:else
      _))
  (return false))

(fn GetObjectTransform
  (bind _itemtostore (Variables|Default|GetItemToStore))
  (bind _attachtocomp (Variables|/Game/GameElementBP/BP_PickupCube.BP_PickupCube_C|GetAttachToComp _itemtostore))
  (bind _returnvalue (Transformation|GetWorldTransform _attachtocomp))
  (return (Class|KismetMathLibrary|TInterpto (Transformation|GetActorTransform (Variables|Default|GetItemToStore)) (Math|Transform|MakeTransform (.location _returnvalue) (.rotation _returnvalue) (Variables|/Game/GameElementBP/BP_PickupCube.BP_PickupCube_C|GetWorldScale _itemtostore)) (Utilities|Time|GetWorldDeltaSeconds) 0.0)))

(fn ResetState
  (Variables|Default|SetShouldStoreItem false)
  (Variables|Default|SetIsSlotUsed false)
  (Variables|/Game/GameElementBP/BP_PickupCube.BP_PickupCube_C|SetCanPickUpItem (Variables|Default|GetItemToStore) true)
  (EventDispatchers|UnbindEventfromOnPickup (Variables|Default|GetItemToStore) (EventDispatchers|CreateEvent :!event Custom|OnItemStoredPickedUp))
  (EventDispatchers|UnbindEventfromOnDrop (Variables|Default|GetItemToStore) (EventDispatchers|CreateEvent :!event Custom|OnItemStoredDropped))
  (Variables|Default|SetItemToStore 0))