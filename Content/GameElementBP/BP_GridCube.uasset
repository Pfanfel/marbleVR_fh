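; Base VR-pickable building cube that snaps to a grid and to neighbouring cubes, glowing when a motion controller hovers over it.
; While held, Tick traces to pickup actors for the nearest cube and previews placement with a ghost, offset from the hit face, rotated in 90-degree steps.
; Released cubes snap beside that neighbour, or wherever physics settles, then get replaced by their "Complex" variant, picked by class name.
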(event OnComponentBeginOverlap(Box)
  (params (OverlappedComponent :type Primitive%20Component%20Object%20Reference) (OtherActor :type Actor%20Object%20Reference) (OtherComp :type Primitive%20Component%20Object%20Reference) (OtherBodyIndex :type Integer) (bFromSweep :type Boolean) (SweepResult :type Hit%20Result%20Structure%20%28by%20ref%29))
  (Utilities|Casting|CastToBP_MotionController OtherActor)
  (Rendering|SetVisibility (Variables|Default|GetHover%20Glow) true false))

(event OnComponentEndOverlap(Box)
  (params (OverlappedComponent :type Primitive%20Component%20Object%20Reference) (OtherActor :type Actor%20Object%20Reference) (OtherComp :type Primitive%20Component%20Object%20Reference) (OtherBodyIndex :type Integer))
  (Utilities|Casting|CastToBP_MotionController OtherActor)
  (Rendering|SetVisibility (Variables|Default|GetHover%20Glow) false false))

(event EventBeginPlay)

(event Collision|EventActorBeginOverlap
  (params (OtherActor :type Actor%20Object%20Reference)))

(event EventTick
  (params (DeltaSeconds :type Float%20%28single-precision%29))
  (bind _spawnedghost (Variables|Default|GetSpawnedGhost))
  (bind _staticmeshcomponent (Variables|/Script/Engine.StaticMeshActor|GetStaticMeshComponent _spawnedghost))
  (if (Variables|Default|GetIsGrabbed)
    (bind (_closestobject _closesthitlocation) (CallFunction|GetClosestCube))
    (Utilities|IsValid _closestobject
      (:Is%20Valid
        (bind (_xoffset _yoffset _zoffset) (CallFunction|GetOffset _closesthitlocation _closestobject))
        (if (Variables|Default|GetIsGhostSpawned)
          _
          (else
            (|SpawnGhost (Transformation|GetActorTransform _closestobject))))
        (Transformation|SetActorTransform (Variables|Default|GetSpawnedGhost) (Transformation|GetActorTransform _closestobject))
        (Transformation|AddActorLocalOffset (Variables|Default|GetSpawnedGhost) (Math|Vector|MakeVector _xoffset _yoffset _zoffset) false false)
        (bind _rotation (CallFunction|CalculateRotation))
        (Transformation|SetWorldRotation (Variables|/Script/Engine.Actor|GetRootComponent _spawnedghost) _rotation false false)
        (bind _location (CallFunction|CalculateSnappedGridLocation _staticmeshcomponent))
        (Transformation|SetWorldLocation _staticmeshcomponent _location false false))
      (:Is%20Not%20Valid
        (CallFunction|DestroyGhost)))
    (else
      (bind _returnvalue (Physics|GetPhysicsLinearVelocity (Variables|Debug|GetStaticMeshComponent) "None"))
      (if (<= (Math|Vector|VectorLength _returnvalue) 0.005)
        (Physics|SetPhysicsLinearVelocity (Variables|Debug|GetStaticMeshComponent) "0, 0, 0" false "None")
        (Class|PrimitiveComponent|SetPhysicsAngularVelocityinDegrees (Variables|Debug|GetStaticMeshComponent) "0, 0, 0" false "None")
        (bind _rotation_2 (CallFunction|CalculateRotation))
        (CallFunction|SnaptoClosestGrid _rotation_2)
        (CallFunction|SpawnComplexVersion)))))

(event EventPickup
  (params (AttachTo :type Scene%20Component%20Object%20Reference))
  (Physics|SetSimulatePhysics (Variables|Debug|GetStaticMeshComponent) false)
  (Transformation|AttachComponentToComponent (VehicleSound|GetRootComponent) AttachTo "None" "KeepWorld" "KeepWorld" "KeepWorld" false)
  (Class|PrimitiveComponent|SetConstraintMode (Variables|Debug|GetStaticMeshComponent) "None")
  (Actor|Tick|SetActorTickEnabled true)
  (Variables|Default|SetIsGrabbed true))

(event EventDrop
  (Variables|Default|SetIsGrabbed false)
  (CallFunction|DestroyGhost)
  (Physics|SetSimulatePhysics (Variables|Debug|GetStaticMeshComponent) true)
  (Transformation|DetachFromActor "KeepWorld" "KeepWorld" "KeepWorld")
  (bind (_closestobject _closesthitlocation) (CallFunction|GetClosestCube))
  (Utilities|IsValid _closestobject
    (:Is%20Valid
      (Physics|SetPhysicsLinearVelocity (Variables|Debug|GetStaticMeshComponent) "0, 0, 0" false "None")
      (Class|PrimitiveComponent|SetPhysicsAngularVelocityinDegrees (Variables|Debug|GetStaticMeshComponent) "0, 0, 0" false "None")
      (bind (_xoffset _yoffset _zoffset) (CallFunction|GetOffset _closesthitlocation _closestobject))
      (bind _rotation (CallFunction|CalculateRotation))
      (Transformation|SetActorTransform (Transformation|GetActorTransform _closestobject))
      (Transformation|AddActorLocalOffset (Math|Vector|MakeVector _xoffset _yoffset _zoffset) false false)
      (CallFunction|SnaptoClosestGrid _rotation)
      (CallFunction|SpawnComplexVersion))
    (:Is%20Not%20Valid
      (Class|PrimitiveComponent|SetConstraintMode (Variables|Debug|GetStaticMeshComponent) "None"))))

(fn ConstructionScript)

(fn CalculateRotation
  (bind _returnvalue (Transformation|GetActorRotation))
  (bind _rotationindegree (CallFunction|ConvertRotationtoRotationinDegree (Math|Float|Round (.roll _returnvalue))))
  (bind _rotationindegree_2 (CallFunction|ConvertRotationtoRotationinDegree (Math|Float|Round (.pitch _returnvalue))))
  (bind _rotationindegree_3 (CallFunction|ConvertRotationtoRotationinDegree (Math|Float|Round (.yaw _returnvalue))))
  (Math|Integer|CompareInt (Math|Integer|%(Integer) _rotationindegree 90) 45
    (:>
      (LocalVariables|SetretX 90 :!label _label))
    (:==
      (goto _label))
    (:<
      (LocalVariables|SetretX 0)))
  (Math|Integer|CompareInt (Math|Integer|%(Integer) _rotationindegree_2 90) 45
    (:>
      (LocalVariables|SetretY 90 :!label _label_2))
    (:==
      (goto _label_2))
    (:<
      (LocalVariables|SetretY 0)))
  (Math|Integer|CompareInt (Math|Integer|%(Integer) _rotationindegree_3 90) 45
    (:>
      (LocalVariables|SetretZ 90 :!label _label_3))
    (:==
      (goto _label_3))
    (:<
      (LocalVariables|SetretZ 0)))
  (return (Math|Rotator|MakeRotator (Math|Conversions|ToFloat(Integer) (+ (LocalVariables|GetretX) (* (/ _rotationindegree 90) 90))) (Math|Conversions|ToFloat(Integer) (+ (LocalVariables|GetretY) (* (/ _rotationindegree_2 90) 90))) (Math|Conversions|ToFloat(Integer) (+ (LocalVariables|GetretZ) (* (/ _rotationindegree_3 90) 90))))))

(fn ConvertRotationtoRotationinDegree
  (params (Rotation :type Integer))
  (Math|Integer|CompareInt (Class|KismetMathLibrary|SignOfInteger Rotation)
    (:>
      (LocalVariables|SetReturnValue Rotation :!label _label))
    (:==
      (goto _label))
    (:<
      (LocalVariables|SetReturnValue (+ (- 180 (Math|Integer|Absolute(Integer) Rotation)) 180))))
  (return (LocalVariables|GetReturnValue)))

(fn CalculateSnappedGridLocation
  (params (StaticMeshComponent :type Static%20Mesh%20Component%20Object%20Reference))
  (bind _returnvalue (Transformation|GetWorldLocation StaticMeshComponent))
  (bind _returnvalue_2 (Math|Float|SnapToGrid(Float) (.z _returnvalue) 1e+01))
  (if (< _returnvalue_2 0.0)
    (LocalVariables|SetretZ 0.0)
    (else
      (LocalVariables|SetretZ _returnvalue_2)))
  (return (Math|Vector|MakeVector (Math|Float|SnapToGrid(Float) (.x _returnvalue) 1e+01) (Math|Float|SnapToGrid(Float) (.y _returnvalue) 1e+01) (LocalVariables|GetretZ))))

(fn GetClosestCube
  (bind _outactors (Actor|GetAllActorswithInterface "/Game/VirtualRealityBP/Blueprints/PickupActorInterface.PickupActorInterface_C"))
  (for _array_element _outactors
    (bind _outhit (Collision|LineTraceForObjects (Transformation|GetActorLocation self) (Transformation|GetActorLocation _array_element) (Utilities|Array|MakeArray "ObjectTypeQuery4") false 0 "None"))
    (if (.bBlockingHit (Collision|BreakHitResult _outhit))
      (if (.bSuccess (Utilities|Casting|CastToBP_GridCube (.HitActor (Collision|BreakHitResult _outhit))))
        ;[1 1 1] Berechnet die Länge von aktuellem Standpunkt zum Hitpunkt
        (bind _output_get (LocalVariables|Set_HitLocation (.Location (Collision|BreakHitResult _outhit))))
        (LocalVariables|Set_CurrDistance (Math|Vector|VectorLength (- _output_get (Transformation|GetActorLocation self))))
        ;[1 1 1] Wenn es der naheste Schnittpunkt ist dann wird das getroffene Objekt und die minimale Distanz gesetzt!
        (if (and (< (LocalVariables|Get_CurrDistance) (LocalVariables|Get_ShortestDistance)) (!= (LocalVariables|Get_CurrDistance) 0.0))
          (bind _returnvalue (CallFunction|GetCubeWidth))
          (if (< (LocalVariables|Get_CurrDistance) (* _returnvalue 1.0))
            (LocalVariables|Set_ClosestObject (.AsBP%20Grid%20Cube (Utilities|Casting|CastToBP_GridCube (.HitActor (Collision|BreakHitResult _outhit)))))
            (LocalVariables|Set_ShortestDistance (LocalVariables|Get_CurrDistance))
            (LocalVariables|Set_ClosestHitLocation (LocalVariables|Get_HitLocation)))))))
  (return (LocalVariables|Get_ClosestObject) (LocalVariables|Get_ClosestHitLocation)))

(fn GetCubeWidth
  (bind _staticmeshcomponent (Variables|Debug|GetStaticMeshComponent))
  (return (* (* (.x (Transformation|GetWorldScale _staticmeshcomponent)) (.x (.Max (Components|StaticMesh|GetLocalBounds _staticmeshcomponent)))) 2.0)))

(fn GetOffset
  (params (HitLocation :type Vector) (ClosestObject :type Actor%20Object%20Reference))
  (bind _returnvalue (Transformation|GetActorTransform ClosestObject))
  (bind _returnvalue_2 (Math|Transform|InverseTransformLocation _returnvalue HitLocation))
  (bind _returnvalue_3 (Math|Float|Absolute(Float) (.x _returnvalue_2)))
  (bind _returnvalue_4 (Math|Float|Absolute(Float) (.y _returnvalue_2)))
  (bind _returnvalue_5 (Math|Float|Absolute(Float) (.z _returnvalue_2)))
  (bind _asbp_grid_cube (Utilities|Casting|CastToBP_GridCube ClosestObject))
  (bind (_xoffset _yoffset _zoffset) (CallFunction|CalculateOffsetsfromHitSide _asbp_grid_cube (.x _returnvalue_2) (.y _returnvalue_2) (.z _returnvalue_2)))
  ;[1 1 1] Calculates the hit side (line trace from Self to Closest Object) and only sets the Offset of the hit side.
  (Math|Float|CompareFloat _returnvalue_3 _returnvalue_4
    (:>
      (Math|Float|CompareFloat _returnvalue_3 _returnvalue_5 :!label _label
        (:>
          (bind _output_get (LocalVariables|Set_XOffset _xoffset :!label _label_2)))
        (:==
          (goto _label_2))
        (:<
          (bind _output_get_2 (LocalVariables|Set_ZOffset _zoffset :!label _label_3)))))
    (:==
      (goto _label))
    (:<
      (Math|Float|CompareFloat _returnvalue_4 _returnvalue_5
        (:>
          (bind _output_get_3 (LocalVariables|Set_YOffset _yoffset)))
        (:==
          (goto _label_3))
        (:<
          (goto _label_3)))))
  (return _output_get _output_get_3 _output_get_2))

(fn CalculateOffsetsfromHitSide
  (params (LocalHitX :type Float%20%28single-precision%29) (LocalHitY :type Float%20%28single-precision%29) (LocalHitZ :type Float%20%28single-precision%29))
  ;[1 1 1] Calculates the offset for all three dimensions.
  (bind _returnvalue (CallFunction|GetCubeWidth))
  (return (* (Math|Float|Sign(Float) LocalHitX) _returnvalue) (* (Math|Float|Sign(Float) LocalHitY) _returnvalue) (* (Math|Float|Sign(Float) LocalHitZ) _returnvalue)))

(fn DestroyGhost
  ;[1 1 1] Destroys the Ghost Actor, when distance is too big again.
  (if (Variables|Default|GetIsGhostSpawned)
    (Actor|DestroyActor (Variables|Default|GetSpawnedGhost))
    (Variables|Default|SetIsGhostSpawned false)))

(fn SnaptoClosestGrid
  (params (NewRotation :type Rotator))
  ;[1 1 1] TODO fuer Y behandeln um nicht aus der Wand raus zu bauen
  (bind _location (CallFunction|CalculateSnappedGridLocation (Variables|Debug|GetStaticMeshComponent)))
  (Transformation|SetWorldLocation (Variables|Debug|GetStaticMeshComponent) _location false false)
  (Transformation|SetWorldRotation (Variables|Debug|GetStaticMeshComponent) NewRotation false false)
  (Class|PrimitiveComponent|SetConstraintMode (Variables|Debug|GetStaticMeshComponent) "Default")
  (Actor|Tick|SetActorTickEnabled false))

(fn SpawnComplexVersion
  (bind _returnvalue (Transformation|GetActorLocation))
  (bind _returnvalue_2 (Transformation|GetActorRotation))
  (bind _returnvalue_3 (Math|Transform|MakeTransform _returnvalue _returnvalue_2))
  (switch string (Utilities|GetClassDisplayName (Utilities|GetClass self))
    (:BP_GridCurveCube_C
      (Game|SpawnActorfromClass "/Game/GameElementBP/Cubes/CurveCube/BP_GridCurveCubeComplex.BP_GridCurveCubeComplex_C" _returnvalue_3 "Undefined" 0 0))
    (:BP_GridEndCube_C
      (Game|SpawnActorfromClass "/Game/GameElementBP/Cubes/EndCube/BP_GridEndCubeComplex.BP_GridEndCubeComplex_C" _returnvalue_3 "Undefined" 0 0))
    (:BP_GridNormalCube_C
      (Game|SpawnActorfromClass "/Game/GameElementBP/Cubes/NormalCube/BP_GridNormalCubeComplex.BP_GridNormalCubeComplex_C" _returnvalue_3 "Undefined" 0 0))
    (:BP_GridStraightCube_C
      (Game|SpawnActorfromClass "/Game/GameElementBP/Cubes/StraightCube/BP_GridStraightCubeComplex.BP_GridStraightCubeComplex_C" _returnvalue_3 "Undefined" 0 0))
    (:BP_GridStraightHalfCube_C
      (Game|SpawnActorfromClass "/Game/GameElementBP/Cubes/StraightHalfCube/BP_GridStraightHalfCubeComplex.BP_GridStraightHalfCubeComplex_C" _returnvalue_3 "Undefined" 0 0))
    (:BP_GridStraightHalfHoleCube_C
      (Game|SpawnActorfromClass "/Game/GameElementBP/Cubes/StraightHalfHoleCube/BP_GridStraightHalfHoleCubeComplex.BP_GridStraightHalfHoleCubeComplex_C" _returnvalue_3 "Undefined" 0 0)))
  (Actor|DestroyActor self))